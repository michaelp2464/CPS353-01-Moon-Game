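; BP_Door2 is a sliding double glass door that opens when its bound OpenDoor event fires.
; BeginPlay binds Activate_door, which plays a sci-fi door sound and runs a timeline lerping both panels apart, with no closing logic.
; A box trigger toggles input for the ThirdPersonCharacter's visit, but no input events exist here and its CanOpen check leads nowhere.
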(event OnComponentEndOverlap(Box)
  (params (OverlappedComponent :type Primitive%20Component%20Object%20Reference) (OtherActor :type Actor%20Object%20Reference) (OtherComp :type Primitive%20Component%20Object%20Reference) (OtherBodyIndex :type Integer))
  (Utilities|Casting|CastToThirdPersonCharacter OtherActor)
  (Input|DisableInput (Game|GetPlayerController 0)))

(event OnComponentBeginOverlap(Box)
  (params (OverlappedComponent :type Primitive%20Component%20Object%20Reference) (OtherActor :type Actor%20Object%20Reference) (OtherComp :type Primitive%20Component%20Object%20Reference) (OtherBodyIndex :type Integer) (bFromSweep :type Boolean) (SweepResult :type Hit%20Result%20Structure%20%28by%20ref%29))
  (Utilities|Casting|CastToThirdPersonCharacter OtherActor)
  (Input|EnableInput (Game|GetPlayerController 0))
  (if (Variables|Default|GetcanOpen)
    _))

(event Custom|Activate_door
  ;[1 1 1] Open the door -Mikey
  ;[1 1 1] Play sound at door location - Mikey
  (Audio|PlaySoundatLocation "/Game/Joshua/Sounds/Slidingdoor_Sounds/Sci-Fi_Sliding_Door_Cue.Sci-Fi_Sliding_Door_Cue" (Transformation|GetWorldLocation (Variables|Default|GetGlassDoorA)) "0, 0, 0" 1.0 1.0 0.0 0 0 0)
  ;[1 1 1] Open the doors by moving each side away from each other - Mikey
  (bind _newtrack_0 (Timeline|Timeline_0 Play)
    (:Update
      (Transformation|SetRelativeLocation (Variables|Default|GetGlassDoorB) (Math|Vector|Lerp(Vector) "0, 0, 0" "170.000000, 0, 0" _newtrack_0) false false)
      (Transformation|SetRelativeLocation (Variables|Default|GetGlassDoorA) (Math|Vector|Lerp(Vector) "-361.000000,69.999992, 0" "-535.000000,69.999878, 0" _newtrack_0) false false))))

(event EventBeginPlay
  (EventDispatchers|BindEventtoOpenDoor (delegate Custom|Activate_door)))

(fn ConstructionScript)