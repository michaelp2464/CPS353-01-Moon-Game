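; Base physics pickup that the player carries on a constraint, with empty hooks for child classes like BP_PickUp_Hard.
; Hits while held free the constraint's linear limits to keep it out of the ground.
; Optionally, a swept proxy mesh follows the main mesh and replaces it visually when walls separate them, preventing pass-through.
; Drop breaks the constraint, exits rotate mode, restores collision and snaps to the proxy if used.
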(event Custom|HitCustom
  (params (HitComponent :type Primitive%20Component%20Object%20Reference) (OtherActor :type Actor%20Object%20Reference) (OtherComp :type Primitive%20Component%20Object%20Reference) (NormalImpulse :type Vector) (Hit :type Hit%20Result%20Structure%20%28by%20ref%29))
  (bind _physicsconstraint (Variables|Default|GetPhysicsConstraint))
  ;[1 1 1] Hit
  (if (not (Variables|Default|GetIgnoreHit?))
    (if (Variables|Default|GetAttach)
      (Variables|Default|SetHitActive true)
      ;;[1 1 1] Prevents the cube from entering the ground
      (Class|PhysicsConstraintComponent|SetLinearXLimit _physicsconstraint "LCM_Free" 0.0)
      (Class|PhysicsConstraintComponent|SetLinearYLimit _physicsconstraint "LCM_Free" 0.0)
      (Class|PhysicsConstraintComponent|SetLinearZLimit _physicsconstraint "LCM_Free" 0.0))))

(event Custom|SweepMeshOff
  ;[1 1 1] Hit
  ;;[0 0 0] FixWallPassThrough
  ;;;[1 1 1] Used in child classes. (BP_PickUp_Hard)
)

(event Custom|Free
  ;[1 1 1] Hit
  ;;[1 1 1] Used in child classes. BP_PickUp_Hard
)

(event Custom|Lock
  ;[1 1 1] Hit
  ;;[1 1 1] Used in child classes. BP_PickUp_Hard
)

(event Custom|SweepMeshHit
  (params (HitComponent :type Primitive%20Component%20Object%20Reference) (OtherActor :type Actor%20Object%20Reference) (OtherComp :type Primitive%20Component%20Object%20Reference) (NormalImpulse :type Vector) (Hit :type Hit%20Result%20Structure%20%28by%20ref%29))
  (bind _mainmash (Variables|Default|GetMainMash))
  (bind _mainmash_2 (Variables|Default|GetMainMash))
  (bind _returnvalue (Transformation|GetWorldLocation _mainmash))
  ;[1 1 1] Hit
  ;;[0 0 0] FixWallPassThrough
  (if (Variables|Default|GetAttach)
    (Utilities|FlowControl|Delay 0.0)
    (if (> (Math|Vector|Distance(Vector) (Transformation|GetWorldLocation (Variables|Default|GetMainMash)) (Transformation|GetWorldLocation (Variables|Default|GetSweepMesh))) 2e+01)
      (Utilities|FlowControl|DoOnce false :!label _label
        (:Completed
          (Variables|Default|SetHit Hit)
          (Utilities|FlowControl|Sequence
            (:then_0
              (Variables|Default|SetFixWallPassActive true)
              (Rendering|SetVisibility (Variables|Default|GetSweepMesh) true false)
              (Rendering|SetVisibility _mainmash_2 false false)
              (Collision|SetCollisionResponsetoAllChannels _mainmash_2 "ECR_Ignore")
              (Variables|Default|SetTickForSweep false))
            (:then_1
              (goto _label_2 Open))
            (:then_2
              (Utilities|FlowControl|Gate true :!label _label_2
                (:Exit
                  (Utilities|FlowControl|Sequence
                    (:then_0
                      (if (and (< (Math|Vector|Distance(Vector) _returnvalue (+ (.ImpactPoint (Collision|BreakHitResult (Variables|Default|GetHit))) (* (.ImpactNormal (Collision|BreakHitResult (Variables|Default|GetHit))) 5.0))) (Math|Vector|Distance(Vector) _returnvalue (.ImpactPoint (Collision|BreakHitResult (Variables|Default|GetHit))))) (> (Math|Vector|Distance(Vector) _returnvalue (.ImpactPoint (Collision|BreakHitResult (Variables|Default|GetHit)))) 25.0)) ; Waiting for MainMesh to return to normal.
                        (Utilities|FlowControl|Sequence
                          (:then_0
                            (Utilities|FlowControl|Sequence
                              (:then_0
                                (goto _label_2 Close))
                              (:then_1
                                (Variables|Default|SetFixWallPassActive false))
                              (:then_2
                                (goto _label Reset))))
                          (:then_1
                            (Rendering|SetVisibility (Variables|Default|GetSweepMesh) false false)
                            (Rendering|SetVisibility (Variables|Default|GetMainMash) true false)))))
                    (:then_1
                      (Utilities|FlowControl|Delay 0.0)
                      (goto _label_2))))))))))))

(event Custom|StopSweep
  (bind _mainmash (Variables|Default|GetMainMash))
  (bind _mainmash_2 (Variables|Default|GetMainMash))
  (bind _returnvalue (Transformation|GetWorldLocation _mainmash))
  ;[1 1 1] Hit
  ;;[0 0 0] FixWallPassThrough
  (Transformation|SetWorldTransform (Variables|Default|GetMainMash) (Transformation|GetWorldTransform (Variables|Default|GetSweepMesh)) false true)
  (Utilities|FlowControl|Sequence
    (:then_0
      (Utilities|FlowControl|Sequence
        (:then_0
          (Utilities|FlowControl|Gate true) ; enters at Close
        )
        (:then_1
          (Variables|Default|SetFixWallPassActive false))
        (:then_2
          (Utilities|FlowControl|DoOnce false) ; enters at Reset
        )))
    (:then_1
      (Rendering|SetVisibility (Variables|Default|GetSweepMesh) false false)
      (Rendering|SetVisibility (Variables|Default|GetMainMash) true false))))

(event Custom|SweepMeshOn
  ;[1 1 1] Hit
  ;;[0 0 0] FixWallPassThrough
  ;;;[1 1 1] Used in child classes. (BP_PickUp_Hard)
)

(event EventBeginPlay
  (bind _root (Variables|Default|GetRoot))
  ;[1 1 1] BeginPlay
  (Utilities|IsValid (Variables|Default|GetPhysicsConstraint)
    (:Is%20Valid
      (Utilities|FlowControl|Sequence
        (:then_0
          (Collision|BindEventtoOnComponentHit (Variables|Default|GetMainMash) (EventDispatchers|CreateEvent :!event Custom|HitCustom))
          (if (Utilities|Enum|Equal(Enum) (Collision|GetCollisionEnabled (Variables|Default|GetMainMash)) "QueryAndPhysics")
            (Physics|SetSimulatePhysics (Variables|Default|GetMainMash) (Variables|A|GetStartPhysics)))
          (Transformation|SetAbsolute _root false true false)
          (Transformation|SetWorldRotation _root "0, 0, 0" false false))
        (:then_1
          (if (Variables|A|GetFixWallPassThrough)
            (Collision|BindEventtoOnComponentHit (Variables|Default|GetSweepMesh) (EventDispatchers|CreateEvent :!event Custom|SweepMeshHit))))))))

(event EventTick
  (params (DeltaSeconds :type Float%20%28single-precision%29))
  ;[1 1 1] EventTick
  (if (and (Variables|Default|GetTickForSweep) (Variables|A|GetFixWallPassThrough))
    (Transformation|SetWorldTransform (Variables|Default|GetSweepMesh) (Transformation|GetWorldTransform (Variables|Default|GetMainMash)) true false)))

(event EventDrop
  (bind _returnvalue (Game|GetPlayerController 0))
  (bind _mainmash (Variables|Default|GetMainMash))
  ;[1 1 1] Drop
  (Utilities|FlowControl|Sequence
    (:then_0
      (if (Variables|A|GetFixWallPassThrough)
        (CallFunction|StopSweep))
      (if (or (Variables|Default|GetRotate) (Audio|Components|Audio|IsPlaying (Variables|Default|GetTimeline_In)))
        (Variables|Default|SetRotate false)
        (Audio|Components|Audio|Stop (Variables|Default|GetTimeline_In))
        (Input|SetIgnoreMoveInput _returnvalue false)
        (Input|SetIgnoreLookInput _returnvalue false)
        (Physics|SetSimulatePhysics _mainmash true)
        (Rendering|SetRenderCustomDepth _mainmash false)
        (Variables|/Script/Engine.PostProcessVolume|SetbEnabled (Variables|Default|GetPP_Playroom (.AsPC%20PIS (Utilities|Casting|CastTo (Game|GetPlayerController 0)))) false))
      (Variables|Default|SetAttach false)
      (Class|PhysicsConstraintComponent|BreakConstraint (Variables|Default|GetPhysicsConstraint))
      (Utilities|FlowControl|Sequence
        (:then_0
          (Utilities|DefaultCollision)
          (Utilities|Array|Clear (Variables|Default|GetIntCollision))
          (Input|DisableInput (Game|GetPlayerController 0))
          (Widget|SetVisibility (Variables|Default|GetCenter (Variables|Default|GetHud (.AsPC%20PIS (Utilities|Casting|CastTo (Game|GetPlayerController 0))))) "SelfHitTestInvisible"))
        (:then_1
          (Utilities|FlowControl|Delay 0.0)
          (Class|PrimitiveComponent|WakeAllRigidBodies (Variables|Default|GetMainMash)))
        (:then_2
          (Utilities|FlowControl|RetriggerableDelay 1.0)
          (if (not (Variables|Default|GetAttach))
            (Variables|Default|SetTickForSweep false)
            (Transformation|DetachFromComponent (Variables|Default|GetRoot) "KeepWorld" "KeepRelative" "KeepWorld" true)))))
    (:then_1
      (Default|CallEDDrop))))

(fn ConstructionScript)

(fn AttachLocation
  (bind _returnvalue (Game|GetPlayerCameraManager 0))
  (bind _offset (Variables|A|GetOffset))
  (bind _transformcomponent (Variables|/Script/Engine.PlayerCameraManager|GetTransformComponent _returnvalue))
  (bind _returnvalue_2 (Transformation|GetWorldLocation _transformcomponent))
  (bind _returnvalue_3 (Math|Vector|GetForwardVector _transformcomponent))
  (return (+ _returnvalue_2 (* _returnvalue_3 (Math|Float|SelectFloat (Math|Vector|Distance(Vector) (- (Transformation|GetWorldLocation (Variables|Default|GetMainMash)) (.Location (Math|Transform|BreakTransform (Variables|Default|GetIntTransform)))) _returnvalue_2) 2.5e+02 (and (Variables|A|GetIgnoreCamera?) (not (Audio|Components|Audio|IsPlaying (Variables|Default|GetTimeline_Out)))))) (+ (* _returnvalue_3 (.x _offset)) (* (Math|Vector|GetRightVector _transformcomponent) (.y _offset)) (* (Math|Vector|GetUpVector _transformcomponent) (.z _offset))))))