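; Interactable telescope actor that lets the player view a star plane through a scope, with input enabled while the third-person character overlaps it.
; Interact toggles the view: it blends to the telescope camera, hides the character mesh and HUD, locks movement and look, and shows the overlay widget and plane.
; While active, mouse axes shift the camera in world X and Z.
; The mouse wheel moves it along world Y to zoom.
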(event Collision|EventActorBeginOverlap
  (params (OtherActor :type Actor%20Object%20Reference))
  ;[1 1 1] Describes when input will be enabled
  (Utilities|Casting|CastToThirdPersonCharacter OtherActor)
  (Input|EnableInput (Game|GetPlayerController 0))
  (Development|PrintString "enter bounding box"))

(event Collision|EventActorEndOverlap
  (params (OtherActor :type Actor%20Object%20Reference))
  ;[1 1 1] Describes when input will be enabled
  (Utilities|Casting|CastToThirdPersonCharacter OtherActor)
  (Input|DisableInput (Game|GetPlayerController 0)))

(event Input|ActionEvents|InputActionInteract
  (params (Key :type Key%20Structure :default "None"))
  (bind _telescope_camera (Variables|Components|GetTelescope_Camera))
  (bind _plane (Variables|Default|GetPlane))
  (:Pressed
    ;[1 1 1] Reset the location of the camera
    (Transformation|SetWorldLocation _telescope_camera (Transformation|GetWorldLocation _telescope_camera) false false)
    ;[1 1 1] Disable Input when player is using telescope
    (Input|DisableInput (Game|GetPlayerController 0))
    (CallFunction|ToggleCamera)
    (if (Variables|Components|Getcamera_state)
      ;[1 1 1] Delay for smooth transition into the telescope
      (Utilities|FlowControl|Delay 0.75)
      ;[1 1 1] Create the scope, add it to the player screen, and then set the star plane visible. Set the input to enable because we want to check if the player wants to look around
      (bind _returnvalue (UserInterface|CreateWidget "/Game/Ben/TelescopeOverlay_Widget.TelescopeOverlay_Widget_C"))
      (bind _output_get (Variables|Default|SetTelescopeOverlay _returnvalue))
      (UserInterface|Viewport|AddtoPlayerScreen _output_get)
      (Rendering|SetVisibility _plane true false)
      (Input|EnableInput (Game|GetPlayerController 0))
      (else
        ;[1 1 1] If the player isn't looking in the telescope, the telescope scope should be removed from the screen, and the star plane should be invisible
        (Widget|RemovefromParent (Variables|Default|GetTelescopeOverlay))
        (Rendering|SetVisibility _plane false false)))))

(event Input|AxisEvents|InputAxisCameraMoveX
  (params (AxisValue :type Float%20%28single-precision%29))
  (bind _telescope_camera (Variables|Components|GetTelescope_Camera))
  (bind _returnvalue (Transformation|GetWorldLocation _telescope_camera))
  (bind (_x _y _z) (Math|Vector|BreakVector _returnvalue))
  ;[1 1 1] Mouse input while interacting with the telescope
  (if (Variables|Components|Getcamera_state)
    (Transformation|SetWorldLocation (Variables|Components|GetTelescope_Camera) (Math|Vector|MakeVector (+ _x AxisValue) _y (+ _z (stale Input|AxisEvents|InputAxisCameraMoveY AxisValue))) false false)))

(event Input|AxisEvents|InputAxisCameraMoveY
  (params (AxisValue :type Float%20%28single-precision%29))
  (bind _telescope_camera (Variables|Components|GetTelescope_Camera))
  (bind _returnvalue (Transformation|GetWorldLocation _telescope_camera))
  (bind (_x _y _z) (Math|Vector|BreakVector _returnvalue))
  ;[1 1 1] Mouse input while interacting with the telescope
  (if (Variables|Components|Getcamera_state)
    (Transformation|SetWorldLocation (Variables|Components|GetTelescope_Camera) (Math|Vector|MakeVector (+ _x (stale Input|AxisEvents|InputAxisCameraMoveX AxisValue)) _y (+ _z AxisValue)) false false)))

(event Input|MouseEvents|MouseWheelUp
  (params (Key :type Key%20Structure :default "None"))
  (bind _telescope_camera (Variables|Components|GetTelescope_Camera))
  (bind _returnvalue (Transformation|GetWorldLocation _telescope_camera))
  (bind (_x _y _z) (Math|Vector|BreakVector _returnvalue))
  ;[1 1 1] Mouse input while interacting with the telescope
  ;;[1 1 1] Zoom in and out
  (:Pressed
    (Transformation|SetWorldLocation (Variables|Components|GetTelescope_Camera) (Math|Vector|MakeVector _x (+ _y 1e+01) _z) false false)))

(event Input|MouseEvents|MouseWheelDown
  (params (Key :type Key%20Structure :default "None"))
  (bind _telescope_camera (Variables|Components|GetTelescope_Camera))
  (bind _returnvalue (Transformation|GetWorldLocation _telescope_camera))
  (bind (_x _y _z) (Math|Vector|BreakVector _returnvalue))
  ;[1 1 1] Mouse input while interacting with the telescope
  ;;[1 1 1] Zoom in and out
  (:Pressed
    (Transformation|SetWorldLocation (Variables|Components|GetTelescope_Camera) (Math|Vector|MakeVector _x (+ _y -1e+01) _z) false false)))

(fn ConstructionScript
  ;[1 1 1] When the object is constructed...
  ;[1 1 1] ...Make sure the plane is invisible...
  (Rendering|SetVisibility (Variables|Default|GetPlane) false false)
  (Variables|Default|SettelescopeCameraLocation (Transformation|GetWorldLocation (Variables|Components|GetTelescope_Camera)))
  ;[1 1 1] The star plane shouldn't exist beyond the player's mind
  (Collision|SetCollisionEnabled (Variables|Default|GetPlane) "NoCollision"))

(fn ToggleCamera
  (bind _returnvalue (Game|GetPlayerController 0))
  (bind _returnvalue_2 (Game|GetPlayerCharacter 0))
  ;[1 1 1] Tell the HUD in ThirdPersonCharacter to disable
  (Default|DisableHUD (Variables|Default|GetCharacter) (not (Variables|Components|Getcamera_state)))
  (bind _output_get (Variables|Components|Setcamera_state (not (Variables|Components|Getcamera_state))))
  (if _output_get
    (Game|Player|SetViewTargetwithBlend _returnvalue (Components|GetOwner (Variables|Components|GetTelescope_Camera)) 0.75 "VTBlend_Linear" 0.0 false)
    (Input|SetIgnoreMoveInput _returnvalue true)
    (Input|SetIgnoreLookInput _returnvalue true)
    (bind _asthird_person_character (Utilities|Casting|CastToThirdPersonCharacter _returnvalue_2))
    (Development|SetHiddeninGame (Variables|/Script/Engine.Character|GetMesh _asthird_person_character) true false)
    (else
      (Game|Player|SetViewTargetwithBlend _returnvalue _returnvalue_2 0.33 "VTBlend_Linear" 0.0 false)
      (Input|ResetIgnoreMoveInput _returnvalue)
      (Input|ResetIgnoreLookInput _returnvalue)
      (bind _asthird_person_character_2 (Utilities|Casting|CastToThirdPersonCharacter _returnvalue_2))
      (Development|SetHiddeninGame (Variables|/Script/Engine.Character|GetMesh _asthird_person_character_2) false false))))