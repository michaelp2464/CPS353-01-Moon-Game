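; Interactable trash Blueprint that lets the player switch to a close-up camera view and click a hidden key to equip it.
; Overlap with the player enables input; Interact toggles a blended view to TrashCamera, disabling HUD, movement and look, hiding the character mesh and showing the cursor.
; Left click traces under the cursor and calls EquipItem when the hit component's display name matches one of two hardcoded key boxes.
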(event Collision|EventActorBeginOverlap
  (params (OtherActor :type Actor%20Object%20Reference))
  ;[1 1 1] Check if Player is in Collision box
  (Utilities|Casting|CastToThirdPersonCharacter OtherActor)
  (Input|EnableInput (Game|GetPlayerController 0)))

(event Collision|EventActorEndOverlap
  (params (OtherActor :type Actor%20Object%20Reference))
  ;[1 1 1] Check if Player is in Collision box
  (Utilities|Casting|CastToThirdPersonCharacter OtherActor)
  (Input|DisableInput (Game|GetPlayerController 0)))

(event Input|ActionEvents|InputActionInteract
  (params (Key :type Key%20Structure :default "None"))
  (bind _returnvalue (Game|GetPlayerController 0))
  ;[1 1 1] Toggle camera and approach it if we press E
  (:Pressed
    (CallFunction|ToggleCamera)
    (if (Variables|Components|Getcamera_state)
      (Variables|/Script/Engine.PlayerController|SetbShowMouseCursor _returnvalue true)
      (else
        (Variables|/Script/Engine.PlayerController|SetbShowMouseCursor _returnvalue false)))))

(event Input|MouseEvents|LeftMouseButton
  (params (Key :type Key%20Structure :default "None"))
  (bind _returnvalue (Game|GetPlayerController 0))
  (bind _array (Utilities|Array|MakeArray "ObjectTypeQuery1" "ObjectTypeQuery2"))
  (bind _hitresult (Class|PlayerController|GetHitResultUnderCursorforObjects _returnvalue _array true))
  (bind _hitcomponent (Collision|BreakHitResult _hitresult))
  (bind _returnvalue_2 (Utilities|GetDisplayName _hitcomponent))
  ;[1 1 1] If left mouse button was clicked, check to see what the cursor clicked on
  (:Pressed
    ;;[1 1 1] Equip item if Key
    (if (or (Utilities|Enum|Equal(Enum) _returnvalue_2 "KeyBP_2.Box") (Utilities|Enum|Equal(Enum) _returnvalue_2 "KeyBP_3.Box"))
      (Default|CallEquipItem))))

(fn ConstructionScript
  (Rendering|SetVisibility (Variables|Components|GetTrash_Camera) false false))

(fn ToggleCamera
  (bind _returnvalue (Game|GetPlayerController 0))
  (bind _returnvalue_2 (Game|GetPlayerCharacter 0))
  ;[1 1 1] Tell the HUD in ThirdPersonCharacter to disable
  (Default|DisableHUD (Variables|Components|GetCharacter) (not (Variables|Components|Getcamera_state)))
  (bind _output_get (Variables|Components|Setcamera_state (not (Variables|Components|Getcamera_state))))
  (if _output_get
    (Game|Player|SetViewTargetwithBlend _returnvalue (Components|GetOwner (Variables|Components|GetTrash_Camera)) 0.75 "VTBlend_Linear" 0.0 false)
    (Input|SetIgnoreMoveInput _returnvalue true)
    (Input|SetIgnoreLookInput _returnvalue true)
    (bind _asthird_person_character (Utilities|Casting|CastToThirdPersonCharacter _returnvalue_2))
    (Development|SetHiddeninGame (Variables|/Script/Engine.Character|GetMesh _asthird_person_character) true false)
    (else
      (Game|Player|SetViewTargetwithBlend _returnvalue _returnvalue_2 0.33 "VTBlend_Linear" 0.0 false)
      (Input|ResetIgnoreMoveInput _returnvalue)
      (Input|ResetIgnoreLookInput _returnvalue)
      (bind _asthird_person_character_2 (Utilities|Casting|CastToThirdPersonCharacter _returnvalue_2))
      (Development|SetHiddeninGame (Variables|/Script/Engine.Character|GetMesh _asthird_person_character_2) false false))))