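; Interactable actor that lets the player open and close a snake minigame widget with E while the ThirdPersonCharacter overlaps it.
; Overlap begin and end enable and disable the actor's input, and E toggles the InCircuitBreaker state and the character's HUD.
; Opening creates a new SnakeGame_w each time, while closing only collapses it.
; WebsiteMode locks move and look input and switches input mode, setting focus before the new widget exists.
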(event Collision|EventActorBeginOverlap
  (params (OtherActor :type Actor%20Object%20Reference))
  (Utilities|Casting|CastToThirdPersonCharacter OtherActor)
  (Input|EnableInput (Game|GetPlayerController 0)))

(event Collision|EventActorEndOverlap
  (params (OtherActor :type Actor%20Object%20Reference))
  (Utilities|Casting|CastToThirdPersonCharacter OtherActor)
  (Input|DisableInput (Game|GetPlayerController 0)))

(event Input|KeyboardEvents|E
  (params (Key :type Key%20Structure :default "None"))
  (:Pressed
    (if (Variables|Default|GetinCircuitBreaker)
      (CallFunction|WebsiteMode false)
      (Widget|SetVisibility (Variables|Default|GetCircuitBreakerWidget) "Collapsed")
      (else
        (CallFunction|WebsiteMode true)
        (bind _returnvalue (UserInterface|CreateWidget "/Game/Ben/snakeGame_w.snakeGame_w_C"))
        (bind _output_get (Variables|Default|SetCircuitBreakerWidget _returnvalue))
        (UserInterface|Viewport|AddtoPlayerScreen _output_get)))
    (bind _output_get_2 (Variables|Default|SetinCircuitBreaker (not (Variables|Default|GetinCircuitBreaker))))
    (Development|PrintString (Utilities|String|ToString(Boolean) (Variables|Default|GetinCircuitBreaker)))
    (Default|DisableHUD (Variables|Default|GetCharacter) _output_get_2)))

(fn ConstructionScript)

(fn WebsiteMode
  (params (inWebsite :type Boolean))
  (bind _returnvalue (Game|GetPlayerController 0))
  (if inWebsite
    (Input|SetIgnoreMoveInput _returnvalue true)
    (Input|SetIgnoreLookInput _returnvalue true)
    (Input|SetInputModeGameandUI (Game|GetPlayerController 0) (Variables|Default|GetCircuitBreakerWidget) "DoNotLock" true)
    (Variables|/Script/Engine.PlayerController|SetbShowMouseCursor (Game|GetPlayerController 0) false)
    (else
      (Input|SetIgnoreMoveInput _returnvalue false)
      (Input|SetIgnoreLookInput _returnvalue false)
      (Input|SetInputModeGameOnly (Game|GetPlayerController 0)))))