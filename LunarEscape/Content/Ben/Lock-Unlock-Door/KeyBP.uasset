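; KeyBP is a key pickup actor that the player equips by pressing Equip while standing inside its Box trigger.
; Box overlaps with ThirdPersonCharacter toggle the key's player input and open or close a Gate that guards the Equip action.
; A successful press sets IsEquipped, plays the pickup sound and calls EquipItem on the linked Character with the key's item number, 0.
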(event OnComponentEndOverlap(Box)
  (params (OverlappedComponent :type Primitive%20Component%20Object%20Reference) (OtherActor :type Actor%20Object%20Reference) (OtherComp :type Primitive%20Component%20Object%20Reference) (OtherBodyIndex :type Integer))
  (Utilities|Casting|CastToThirdPersonCharacter OtherActor)
  (Input|DisableInput (Game|GetPlayerController 0))
  (Utilities|FlowControl|Gate true) ; enters at Close
)

(event OnComponentBeginOverlap(Box)
  (params (OverlappedComponent :type Primitive%20Component%20Object%20Reference) (OtherActor :type Actor%20Object%20Reference) (OtherComp :type Primitive%20Component%20Object%20Reference) (OtherBodyIndex :type Integer) (bFromSweep :type Boolean) (SweepResult :type Hit%20Result%20Structure%20%28by%20ref%29))
  (Utilities|Casting|CastToThirdPersonCharacter OtherActor)
  (Input|EnableInput (Game|GetPlayerController 0))
  (Utilities|FlowControl|Gate true) ; enters at Open
)

(event Input|ActionEvents|InputActionEquip
  (params (Key :type Key%20Structure :default "None"))
  (:Pressed
    (Utilities|FlowControl|Gate true
      (:Exit
        (Variables|Default|SetisEquipped true)
        (Audio|PlaySoundatLocation "/Game/Ben/Lock-Unlock-Door/key_pickup.key_pickup" (Transformation|GetActorLocation) "0, 0, 0" 1.0 1.0 0.0 0 0 0)
        ;[1 1 1] Since the Character and this keyBP are linked, keyBP can call the Character's functions
        ;;[1 1 1] Key's num is 0
        (Default|EquipItem (Variables|Default|GetCharacter))))))

(fn ConstructionScript)