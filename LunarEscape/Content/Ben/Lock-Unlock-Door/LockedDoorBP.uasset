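; LockedDoorBP is a door that the player can open and close with Interact, provided the ThirdPersonCharacter has a key.
; A box overlap enables input and opens a gate, and leaving the box reverses both.
; With a key, a FlipFlop alternately plays and reverses a timeline that lerps door yaw, with an opening sound each time.
; Timeline updates disable input, while keyless presses play a locked sound.
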(event OnComponentEndOverlap(Box)
  (params (OverlappedComponent :type Primitive%20Component%20Object%20Reference) (OtherActor :type Actor%20Object%20Reference) (OtherComp :type Primitive%20Component%20Object%20Reference) (OtherBodyIndex :type Integer))
  ;[1 1 1] If the player is within range and has the key...
  (Utilities|Casting|CastToThirdPersonCharacter OtherActor)
  (Input|DisableInput (Game|GetPlayerController 0))
  (Utilities|FlowControl|Gate true) ; enters at Close
)

(event OnComponentBeginOverlap(Box)
  (params (OverlappedComponent :type Primitive%20Component%20Object%20Reference) (OtherActor :type Actor%20Object%20Reference) (OtherComp :type Primitive%20Component%20Object%20Reference) (OtherBodyIndex :type Integer) (bFromSweep :type Boolean) (SweepResult :type Hit%20Result%20Structure%20%28by%20ref%29))
  ;[1 1 1] If the player is within range and has the key...
  (bind _asthird_person_character (Utilities|Casting|CastToThirdPersonCharacter OtherActor))
  (Input|EnableInput (Game|GetPlayerController 0))
  (Utilities|FlowControl|Gate true) ; enters at Open
)

(event Input|ActionEvents|InputActionInteract
  (params (Key :type Key%20Structure :default "None"))
  ;[1 1 1] If the player is within range and has the key...
  (:Pressed
    (if (Variables|/Game/ThirdPersonBP/Blueprints/ThirdPersonCharacter.ThirdPersonCharacter_C|GetHasKey (stale OnComponentBeginOverlap(Box) _asthird_person_character))
      (Utilities|FlowControl|Gate true
        (:Exit
          (Audio|PlaySoundatLocation "/Game/Ben/Lock-Unlock-Door/door_open.door_open" (Transformation|GetActorLocation) "0, 0, 0" 1.0 1.0 0.65 0 0 0)
          ;[1 1 1] ...run the door opening animation
          (Utilities|FlowControl|FlipFlop
            (:A
              ;;[1 1 1] Open/Open animation backwards
              (bind _door_open_close (Timeline|Open/Close%20Door Play)
                (:Update
                  (Transformation|SetRelativeRotation (Variables|Default|GetDoor) (Math|Rotator|MakeRotator 0.0 0.0 (Math|Float|Lerp (Variables|Default|GetClosed) (Variables|Default|GetOpen) _door_open_close)) false false)
                  (Input|DisableInput (Game|GetPlayerController 0)))))
            (:B
              (Timeline|Open/Close%20Door Reverse)))))
      (else
        (Audio|PlaySoundatLocation "/Game/Ben/Lock-Unlock-Door/door_locked.door_locked" (Transformation|GetActorLocation) "0, 0, 0" 1.0 1.0 0.0 0 0 0)))))

(fn ConstructionScript)