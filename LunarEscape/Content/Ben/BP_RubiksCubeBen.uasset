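; BP_RubiksCubeBen is an interactive Rubik's cube with a puzzle-solving mode that can be equipped as an item once solved.
; Box overlap enables input and opens a gate, letting the Equip action equip the cube when IsSolved is set.
; CubeSolveMode toggles solving: a timeline lerps the physics cube to camera height, the character watches it, and movement and look lock while the cursor shows.
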(event OnComponentEndOverlap(BoxCollision)
  (params (OverlappedComponent :type Primitive%20Component%20Object%20Reference) (OtherActor :type Actor%20Object%20Reference) (OtherComp :type Primitive%20Component%20Object%20Reference) (OtherBodyIndex :type Integer))
  ;[1 1 1] Everything I changed is in this box -Ben
  (Utilities|Casting|CastToThirdPersonCharacter OtherActor)
  (Input|DisableInput (Game|GetPlayerController 0))
  (Utilities|FlowControl|Gate true) ; enters at Close
)

(event OnComponentBeginOverlap(BoxCollision)
  (params (OverlappedComponent :type Primitive%20Component%20Object%20Reference) (OtherActor :type Actor%20Object%20Reference) (OtherComp :type Primitive%20Component%20Object%20Reference) (OtherBodyIndex :type Integer) (bFromSweep :type Boolean) (SweepResult :type Hit%20Result%20Structure%20%28by%20ref%29))
  ;[1 1 1] Everything I changed is in this box -Ben
  (Utilities|Casting|CastToThirdPersonCharacter OtherActor)
  (Input|EnableInput (Game|GetPlayerController 0))
  (Utilities|FlowControl|Gate true) ; enters at Open
)

(event Custom|setSolveModeOff
  (bind _returnvalue (Game|GetPlayerController 0))
  ;[1 1 1] Sets character back to normal to leave puzzle-solving position
  (Input|ResetIgnoreLookInput _returnvalue)
  (Input|ResetIgnoreMoveInput _returnvalue)
  (Variables|/Script/Engine.PlayerController|SetbShowMouseCursor _returnvalue false)
  (Variables|Default|SetisInCubeSolveMode false))

(event Custom|setSolveModeOn
  (bind _returnvalue (Game|GetPlayerController 0))
  (bind _cubea (Variables|Default|GetCubeA))
  (bind _returnvalue_2 (Transformation|GetWorldLocation _cubea))
  (bind (_x _y) (Math|Vector|BreakVector _returnvalue_2))
  ;[1 1 1] Sets up camera and Rubiks cube position to solve the puzzle
  (bind _newtrack (Timeline|Timeline_0 PlayFromStart)
    (:Update
      (Transformation|SetWorldLocation (Variables|Default|GetCubeA) (Math|Vector|Lerp(Vector) _returnvalue_2 (Math|Vector|MakeVector _x _y (.Z (Math|Vector|BreakVector (Camera|GetCameraLocation (Game|GetPlayerCameraManager 0))))) _newtrack) false false)
      (bind _asthird_person_character (Utilities|Casting|CastToThirdPersonCharacter (Game|GetPlayerCharacter 0)))
      (Default|WatchObject _asthird_person_character self)
      (Input|SetIgnoreMoveInput _returnvalue true)
      (Input|SetIgnoreLookInput _returnvalue true)
      (Variables|/Script/Engine.PlayerController|SetbShowMouseCursor _returnvalue true)
      (Variables|Default|SetisInCubeSolveMode true))))

(event Input|ActionEvents|InputActionEquip
  (params (Key :type Key%20Structure :default "None"))
  ;[1 1 1] Everything I changed is in this box -Ben
  (:Pressed
    (Utilities|FlowControl|Gate true
      (:Exit
        ;;[1 1 1] isSolved is set to true on default
        (if (Variables|Default|GetisSolved)
          (Variables|Default|SetisEquipped true)
          (Default|EquipItem (Variables|Default|GetCharacter) 1))))))

(fn ConstructionScript
  (Physics|SetSimulatePhysics (Variables|Default|GetCubeA) true))

(fn CubeSolveMode
  ;[1 1 1] Toggle function for Rubiks cube "puzzle solving mode"
  (if (Variables|Default|GetisInCubeSolveMode)
    (CallFunction|SetSolveModeOff)
    (else
      (CallFunction|SetSolveModeon))))