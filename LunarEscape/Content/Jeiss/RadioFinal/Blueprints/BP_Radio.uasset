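; Interactable radio actor that opens a sine puzzle and, once that puzzle is solved, plays static containing the answer.
; A box collision enables the actor's input only while the third-person character overlaps it.
; Pressing E shows the puzzle widget created at BeginPlay with the mouse cursor, toggling the character's HUD.
; If the widget's target is already reached, E plays the answer sound and blocks input during a fixed delay.
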(event OnComponentBeginOverlap(BoxCollision)
  (params (OverlappedComponent :type Primitive%20Component%20Object%20Reference) (OtherActor :type Actor%20Object%20Reference) (OtherComp :type Primitive%20Component%20Object%20Reference) (OtherBodyIndex :type Integer) (bFromSweep :type Boolean) (SweepResult :type Hit%20Result%20Structure%20%28by%20ref%29))
  (Utilities|Casting|CastToThirdPersonCharacter OtherActor)
  (Input|EnableInput (Game|GetPlayerController 0)))

(event OnComponentEndOverlap(BoxCollision)
  (params (OverlappedComponent :type Primitive%20Component%20Object%20Reference) (OtherActor :type Actor%20Object%20Reference) (OtherComp :type Primitive%20Component%20Object%20Reference) (OtherBodyIndex :type Integer))
  (Utilities|Casting|CastToThirdPersonCharacter OtherActor)
  (Input|DisableInput (Game|GetPlayerController 0)))

(event Collision|EventActorBeginOverlap
  (params (OtherActor :type Actor%20Object%20Reference)))

(event EventTick
  (params (DeltaSeconds :type Float%20%28single-precision%29)))

(event EventBeginPlay
  ;[1 1 1] Comment
  (bind _returnvalue (UserInterface|CreateWidget "/Game/Jeiss/RadioFinal/Blueprints/BP_SinPuzzle.BP_SinPuzzle_C")))

(event Input|KeyboardEvents|E
  (params (Key :type Key%20Structure :default "None"))
  (bind _character (Variables|Default|GetCharacter))
  ;[1 1 1] Comment
  (:Pressed
    (Default|DisableHUD _character true)
    (if (Variables|/Game/Jeiss/RadioFinal/Blueprints/BP_SinPuzzle.BP_SinPuzzle_C|GetTargetReached (stale EventBeginPlay _returnvalue))
      (Default|DisableHUD _character false)
      (Audio|PlaySoundatLocation "/Game/Jeiss/RadioFinal/Sound/RadioStaticwithAnswer_Cue.RadioStaticwithAnswer_Cue" (Transformation|GetWorldLocation (Variables|Default|GetRadio)) "0, 0, 0" 1.0 1.0 0.0 0 0 0)
      (Input|DisableInput (Game|GetPlayerController 0))
      (Utilities|FlowControl|Delay 14.0)
      (Input|EnableInput 0)
      (else
        (UserInterface|Viewport|AddtoViewport (stale EventBeginPlay _returnvalue) 0)
        (Variables|/Script/Engine.PlayerController|SetbShowMouseCursor (Game|GetPlayerController 0) true)))))

(fn ConstructionScript)