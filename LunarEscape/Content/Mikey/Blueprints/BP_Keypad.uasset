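; Interactive keypad actor that activates its referenced door when the player enters that door's four-digit code.
; Overlap enables input, and E toggles a blended keypad camera that locks movement and look, shows the cursor and hides character and HUD.
; Widget component buttons fill four digit slots tracked by Init flags, each lighting an indicator.
; Back clears the last slot, and Enter compares digits with the door's code, clearing all on mismatch.
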(event Custom|OnClicked_Button1
  ;[1 1 1] Enter and initialze the next number when a number key is pressed - Mikey
  (CallFunction|EnterNumber 1)
  (CallFunction|InitializeNumber))

(event Custom|OnClicked_Button7
  ;[1 1 1] Enter and initialze the next number when a number key is pressed - Mikey
  (CallFunction|EnterNumber 7)
  (CallFunction|InitializeNumber))

(event Custom|OnClicked_Button6
  ;[1 1 1] Enter and initialze the next number when a number key is pressed - Mikey
  (CallFunction|EnterNumber 6)
  (CallFunction|InitializeNumber))

(event Custom|OnClicked_Button4
  ;[1 1 1] Enter and initialze the next number when a number key is pressed - Mikey
  (CallFunction|EnterNumber 4)
  (CallFunction|InitializeNumber))

(event Custom|OnClicked_Button0
  ;[1 1 1] Enter and initialze the next number when a number key is pressed - Mikey
  (CallFunction|EnterNumber)
  (CallFunction|InitializeNumber))

(event Custom|OnClicked_ButtonBack
  ;[1 1 1] Backspace the last number when the back key is pressed - Mikey
  (CallFunction|Back))

(event Custom|OnClicked_ButtonEnter
  ;[1 1 1] Check if the password is correct when the enter key is pressed - Mikey
  (CallFunction|Enter))

(event Custom|OnClicked_Button2
  ;[1 1 1] Enter and initialze the next number when a number key is pressed - Mikey
  (CallFunction|EnterNumber 2)
  (CallFunction|InitializeNumber))

(event Custom|OnClicked_Button5
  ;[1 1 1] Enter and initialze the next number when a number key is pressed - Mikey
  (CallFunction|EnterNumber 5)
  (CallFunction|InitializeNumber))

(event Custom|OnClicked_Button9
  ;[1 1 1] Enter and initialze the next number when a number key is pressed - Mikey
  (CallFunction|EnterNumber 9)
  (CallFunction|InitializeNumber))

(event Custom|OnClicked_Button3
  ;[1 1 1] Enter and initialze the next number when a number key is pressed - Mikey
  (CallFunction|EnterNumber 3)
  (CallFunction|InitializeNumber))

(event Custom|OnClicked_Button8
  ;[1 1 1] Enter and initialze the next number when a number key is pressed - Mikey
  (CallFunction|EnterNumber 8)
  (CallFunction|InitializeNumber))

(event Collision|EventActorBeginOverlap
  (params (OtherActor :type Actor%20Object%20Reference))
  ;[1 1 1] Enable player input when the player is within range of the keypad - Mikey
  (Utilities|Casting|CastToThirdPersonCharacter OtherActor)
  (Input|EnableInput (Game|GetPlayerController 0)))

(event Collision|EventActorEndOverlap
  (params (OtherActor :type Actor%20Object%20Reference))
  ;[1 1 1] Enable player input when the player is within range of the keypad - Mikey
  (Utilities|Casting|CastToThirdPersonCharacter OtherActor)
  (Input|DisableInput (Game|GetPlayerController 0)))

(event EventBeginPlay
  ;[1 1 1] Make sure each number is deinitialized at the start - Mikey
  (Variables|Default|Setnum2_init false)
  (Variables|Default|Setnum2_init false)
  (Variables|Default|Setnum3_init false)
  (Variables|Default|Setnum4_init false)
  ;[1 1 1] Enter and initialze the next number when a number key is pressed - Mikey
  (bind _aswidget_keypad (Utilities|Casting|CastToWidget_Keypad (UserInterface|GetWidget (Variables|Default|Getbutton_widget))))
  (EventDispatchers|BindEventtoOnClicked (Variables|/Game/Mikey/Blueprints/Widget_Keypad.Widget_Keypad_C|GetButton_1 _aswidget_keypad) (delegate Custom|OnClicked_Button1))
  (EventDispatchers|AssignOnClicked (Variables|/Game/Mikey/Blueprints/Widget_Keypad.Widget_Keypad_C|GetButton_2 _aswidget_keypad) (delegate Custom|OnClicked_Button2))
  (EventDispatchers|AssignOnClicked (Variables|/Game/Mikey/Blueprints/Widget_Keypad.Widget_Keypad_C|GetButton_3 _aswidget_keypad) (delegate Custom|OnClicked_Button3))
  (EventDispatchers|AssignOnClicked (Variables|/Game/Mikey/Blueprints/Widget_Keypad.Widget_Keypad_C|GetButton_4 _aswidget_keypad) (delegate Custom|OnClicked_Button4))
  (EventDispatchers|AssignOnClicked (Variables|/Game/Mikey/Blueprints/Widget_Keypad.Widget_Keypad_C|GetButton_5 _aswidget_keypad) (delegate Custom|OnClicked_Button5))
  (EventDispatchers|AssignOnClicked (Variables|/Game/Mikey/Blueprints/Widget_Keypad.Widget_Keypad_C|GetButton_6 _aswidget_keypad) (delegate Custom|OnClicked_Button6))
  (EventDispatchers|AssignOnClicked (Variables|/Game/Mikey/Blueprints/Widget_Keypad.Widget_Keypad_C|GetButton_7 _aswidget_keypad) (delegate Custom|OnClicked_Button7))
  (EventDispatchers|AssignOnClicked (Variables|/Game/Mikey/Blueprints/Widget_Keypad.Widget_Keypad_C|GetButton_8 _aswidget_keypad) (delegate Custom|OnClicked_Button8))
  (EventDispatchers|AssignOnClicked (Variables|/Game/Mikey/Blueprints/Widget_Keypad.Widget_Keypad_C|GetButton_9 _aswidget_keypad) (delegate Custom|OnClicked_Button9))
  (EventDispatchers|AssignOnClicked (Variables|/Game/Mikey/Blueprints/Widget_Keypad.Widget_Keypad_C|GetButton_0 _aswidget_keypad) (delegate Custom|OnClicked_Button0))
  ;[1 1 1] Backspace the last number when the back key is pressed - Mikey
  (EventDispatchers|AssignOnClicked (Variables|/Game/Mikey/Blueprints/Widget_Keypad.Widget_Keypad_C|GetButton_back _aswidget_keypad) (delegate Custom|OnClicked_ButtonBack))
  ;[1 1 1] Check if the password is correct when the enter key is pressed - Mikey
  (EventDispatchers|AssignOnClicked (Variables|/Game/Mikey/Blueprints/Widget_Keypad.Widget_Keypad_C|GetButton_enter _aswidget_keypad) (delegate Custom|OnClicked_ButtonEnter)))

(event Input|KeyboardEvents|E
  (params (Key :type Key%20Structure :default "None"))
  ;[1 1 1] Toggle the camera when the player presses E - Mikey
  (:Pressed
    (CallFunction|ToggleCamera)))

(fn ConstructionScript)

(fn ToggleCamera
  (bind _returnvalue (Game|GetPlayerController 0))
  (bind _returnvalue_2 (Game|GetPlayerCharacter 0))
  ;[1 1 1] Toggle the camera state -Mikey
  (bind _output_get (Variables|Default|Setcamera_state (not (Variables|Default|Getcamera_state))))
  ;[1 1 1] When the camera is enabled, disable player movement and look input - Mikey
  (if _output_get
    (Game|Player|SetViewTargetwithBlend _returnvalue (Components|GetOwner (Variables|Default|GetKeypad_camera)) 0.75 "VTBlend_Linear" 0.0 false)
    (Input|SetIgnoreMoveInput _returnvalue true)
    (Input|SetIgnoreLookInput _returnvalue true)
    ;[1 1 1] Show the mouse, hide the player model and HUD - Mikey
    (Variables|/Script/Engine.PlayerController|SetbShowMouseCursor _returnvalue true)
    (bind _asthird_person_character (Utilities|Casting|CastToThirdPersonCharacter _returnvalue_2))
    (Development|SetHiddeninGame (Variables|/Script/Engine.Character|GetMesh _asthird_person_character) true false)
    (Default|DisableHUD _asthird_person_character true)
    (else
      ;[1 1 1] When the camera is disabled, enable player movement and look input - Mikey
      (Game|Player|SetViewTargetwithBlend _returnvalue _returnvalue_2 0.33 "VTBlend_Linear" 0.0 false)
      (Input|ResetIgnoreMoveInput _returnvalue)
      (Input|ResetIgnoreLookInput _returnvalue)
      ;[1 1 1] Hide the mouse, show the player model and HUD - Mikey
      (Variables|/Script/Engine.PlayerController|SetbShowMouseCursor _returnvalue false)
      (bind _asthird_person_character_2 (Utilities|Casting|CastToThirdPersonCharacter _returnvalue_2))
      (Development|SetHiddeninGame (Variables|/Script/Engine.Character|GetMesh _asthird_person_character_2) false false)
      (Default|DisableHUD _asthird_person_character_2 false))))

(fn InitializeNumber
  ;[1 1 1] Check for the first uninitialized number and initialize it - Mikey
  (bind _aswidget_keypad (Utilities|Casting|CastToWidget_Keypad (UserInterface|GetWidget (Variables|Default|Getbutton_widget))))
  (if (Variables|Default|Getnum1_init)
    (if (Variables|Default|Getnum2_init)
      (if (Variables|Default|Getnum3_init)
        (if (not (Variables|Default|Getnum4_init))
          (Variables|Default|Setnum4_init true)
          ;[1 1 1] Turn on the light for the initialized number - Mikey
          (Appearance|SetColorandOpacity (Variables|/Game/Mikey/Blueprints/Widget_Keypad.Widget_Keypad_C|Getlight4 _aswidget_keypad) "(R=0.000000,G=1.000000,B=0.124603,A=1.000000)" :!class /Script/UMG.Image))
        (else
          (Variables|Default|Setnum3_init true)
          (Appearance|SetColorandOpacity (Variables|/Game/Mikey/Blueprints/Widget_Keypad.Widget_Keypad_C|Getlight3 _aswidget_keypad) "(R=0.000000,G=1.000000,B=0.124603,A=1.000000)" :!class /Script/UMG.Image)))
      (else
        (Variables|Default|Setnum2_init true)
        (Appearance|SetColorandOpacity (Variables|/Game/Mikey/Blueprints/Widget_Keypad.Widget_Keypad_C|Getlight2 _aswidget_keypad) "(R=0.000000,G=1.000000,B=0.124603,A=1.000000)" :!class /Script/UMG.Image)))
    (else
      (Variables|Default|Setnum1_init true)
      (Appearance|SetColorandOpacity (Variables|/Game/Mikey/Blueprints/Widget_Keypad.Widget_Keypad_C|Getlight1 _aswidget_keypad) "(R=0.000000,G=1.000000,B=0.124603,A=1.000000)" :!class /Script/UMG.Image))))

(fn EnterNumber
  (params (num :type Integer))
  ;[1 1 1] Set the number of the first uninitialized number to the input digit - Mikey
  (if (Variables|Default|Getnum1_init)
    (if (Variables|Default|Getnum2_init)
      (if (Variables|Default|Getnum3_init)
        (if (not (Variables|Default|Getnum4_init))
          (Variables|Default|Setnum4 num))
        (else
          (Variables|Default|Setnum3 num)))
      (else
        (Variables|Default|Setnum2 num)))
    (else
      (Variables|Default|Setnum1 num))))

(fn Back
  ;[1 1 1] Check for the last initialized number and deinitialize it - Mikey
  (bind _aswidget_keypad (Utilities|Casting|CastToWidget_Keypad (UserInterface|GetWidget (Variables|Default|Getbutton_widget))))
  (if (Variables|Default|Getnum4_init)
    (Variables|Default|Setnum4_init false)
    ;[1 1 1] Turn off the light for the deinitialized number - Mikey
    (Appearance|SetColorandOpacity (Variables|/Game/Mikey/Blueprints/Widget_Keypad.Widget_Keypad_C|Getlight4 _aswidget_keypad) "(R=0.000000,G=0.000000,B=0.000000,A=0.000000)" :!class /Script/UMG.Image)
    (elif (Variables|Default|Getnum3_init)
      (Variables|Default|Setnum3_init false)
      (Appearance|SetColorandOpacity (Variables|/Game/Mikey/Blueprints/Widget_Keypad.Widget_Keypad_C|Getlight3 _aswidget_keypad) "(R=0.000000,G=0.000000,B=0.000000,A=0.000000)" :!class /Script/UMG.Image)
      (elif (Variables|Default|Getnum2_init)
        (Variables|Default|Setnum2_init false)
        (Appearance|SetColorandOpacity (Variables|/Game/Mikey/Blueprints/Widget_Keypad.Widget_Keypad_C|Getlight2 _aswidget_keypad) "(R=0.000000,G=0.000000,B=0.000000,A=0.000000)" :!class /Script/UMG.Image)
        (elif (Variables|Default|Getnum1_init)
          (Variables|Default|Setnum1_init false)
          (Appearance|SetColorandOpacity (Variables|/Game/Mikey/Blueprints/Widget_Keypad.Widget_Keypad_C|Getlight1 _aswidget_keypad) "(R=0.000000,G=0.000000,B=0.000000,A=0.000000)" :!class /Script/UMG.Image))))))

(fn Enter
  (bind _door_refer (Variables|Default|Getdoor_refer))
  ;[1 1 1] If the password is correct, open the door - Mikey
  (if (Math|Boolean|ANDBoolean (== (Variables|Default|Getnum1) (Variables|/Game/Mikey/Blueprints/BP_Door_to_open.BP_Door_to_open_C|Getcodenum1 _door_refer)) (== (Variables|Default|Getnum2) (Variables|/Game/Mikey/Blueprints/BP_Door_to_open.BP_Door_to_open_C|Getcodenum2 _door_refer)) (== (Variables|Default|Getnum3) (Variables|/Game/Mikey/Blueprints/BP_Door_to_open.BP_Door_to_open_C|Getcodenum3 _door_refer)) (== (Variables|Default|Getnum4) (Variables|/Game/Mikey/Blueprints/BP_Door_to_open.BP_Door_to_open_C|Getcodenum4 _door_refer)))
    (Default|ActivateDoor (Variables|Default|Getdoor_refer))
    (else
      ;[1 1 1] If the password is incorrect, deinitialize each number on the keypad - Mikey
      (Variables|Default|Setnum1_init false)
      (Variables|Default|Setnum2_init false)
      (Variables|Default|Setnum3_init false)
      (Variables|Default|Setnum4_init false)
      ;[1 1 1] Turn off the light for each keypad number - Mikey
      (bind _aswidget_keypad (Utilities|Casting|CastToWidget_Keypad (UserInterface|GetWidget (Variables|Default|Getbutton_widget))))
      (Appearance|SetColorandOpacity (Variables|/Game/Mikey/Blueprints/Widget_Keypad.Widget_Keypad_C|Getlight1 _aswidget_keypad) "(R=0.000000,G=0.000000,B=0.000000,A=0.000000)" :!class /Script/UMG.Image)
      (Appearance|SetColorandOpacity (Variables|/Game/Mikey/Blueprints/Widget_Keypad.Widget_Keypad_C|Getlight2 _aswidget_keypad) "(R=0.000000,G=0.000000,B=0.000000,A=0.000000)" :!class /Script/UMG.Image)
      (Appearance|SetColorandOpacity (Variables|/Game/Mikey/Blueprints/Widget_Keypad.Widget_Keypad_C|Getlight3 _aswidget_keypad) "(R=0.000000,G=0.000000,B=0.000000,A=0.000000)" :!class /Script/UMG.Image)
      (Appearance|SetColorandOpacity (Variables|/Game/Mikey/Blueprints/Widget_Keypad.Widget_Keypad_C|Getlight4 _aswidget_keypad) "(R=0.000000,G=0.000000,B=0.000000,A=0.000000)" :!class /Script/UMG.Image))))