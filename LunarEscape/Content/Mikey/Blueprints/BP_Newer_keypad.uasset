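; Interactive four-digit keypad that activates its linked door when the entered code matches that door's code numbers.
; While the third-person character overlaps it, E toggles a blended view to the keypad camera, locking move and look, showing the cursor and hiding the character mesh.
; Widget component buttons fill four digit slots tracked by init flags.
; Back clears the last flag; Enter compares digits, clearing all flags on mismatch.
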(event Custom|OnClicked_Button1
  (CallFunction|EnterNumber 1)
  (CallFunction|InitializeNumber))

(event Custom|OnClicked_Button7
  (CallFunction|EnterNumber 7)
  (CallFunction|InitializeNumber))

(event Custom|OnClicked_Button6
  (CallFunction|EnterNumber 6)
  (CallFunction|InitializeNumber))

(event Custom|OnClicked_Button4
  (CallFunction|EnterNumber 4)
  (CallFunction|InitializeNumber))

(event Custom|OnClicked_Button0
  (CallFunction|EnterNumber)
  (CallFunction|InitializeNumber))

(event Custom|OnClicked_ButtonBack
  (if (Variables|Default|Getnum4_init)
    (Variables|Default|Setnum4_init false)
    (elif (Variables|Default|Getnum3_init)
      (Variables|Default|Setnum3_init false)
      (elif (Variables|Default|Getnum2_init)
        (Variables|Default|Setnum2_init false)
        (elif (Variables|Default|Getnum1_init)
          (Variables|Default|Setnum1_init false))))))

(event Custom|OnClicked_ButtonEnter
  (if (Math|Boolean|ANDBoolean (== (Variables|Default|Getnum1) (Variables|/Game/Mikey/Blueprints/Door_to_open.Door_to_open_C|Getcodenum1 (Variables|Default|Getdoor_refer))) (== (Variables|Default|Getnum2) (Variables|/Game/Mikey/Blueprints/Door_to_open.Door_to_open_C|Getcodenum2 (Variables|Default|Getdoor_refer))) (== (Variables|Default|Getnum3) (Variables|/Game/Mikey/Blueprints/Door_to_open.Door_to_open_C|Getcodenum3 (Variables|Default|Getdoor_refer))) (== (Variables|Default|Getnum4) (Variables|/Game/Mikey/Blueprints/Door_to_open.Door_to_open_C|Getcodenum4 (Variables|Default|Getdoor_refer))))
    (Default|ActivateDoor (Variables|Default|Getdoor_refer))
    (else
      (Variables|Default|Setnum1_init false)
      (Variables|Default|Setnum2_init false)
      (Variables|Default|Setnum3_init false)
      (Variables|Default|Setnum4_init false))))

(event Custom|OnClicked_Button2
  (CallFunction|EnterNumber 2)
  (CallFunction|InitializeNumber))

(event Custom|OnClicked_Button5
  (CallFunction|EnterNumber 5)
  (CallFunction|InitializeNumber))

(event Custom|OnClicked_Button9
  (CallFunction|EnterNumber 9)
  (CallFunction|InitializeNumber))

(event Custom|OnClicked_Button3
  (CallFunction|EnterNumber 3)
  (CallFunction|InitializeNumber))

(event Custom|OnClicked_Button8
  (CallFunction|EnterNumber 8)
  (CallFunction|InitializeNumber))

(event Collision|EventActorBeginOverlap
  (params (OtherActor :type Actor%20Object%20Reference))
  (Utilities|Casting|CastToThirdPersonCharacter OtherActor)
  (Input|EnableInput (Game|GetPlayerController 0)))

(event Collision|EventActorEndOverlap
  (params (OtherActor :type Actor%20Object%20Reference))
  (Utilities|Casting|CastToThirdPersonCharacter OtherActor)
  (Input|DisableInput (Game|GetPlayerController 0)))

(event EventBeginPlay
  (Variables|Default|Setnum2_init false)
  (Variables|Default|Setnum2_init false)
  (Variables|Default|Setnum3_init false)
  (Variables|Default|Setnum4_init false)
  (bind _aswidget_newer_keypad (Utilities|Casting|CastToWidget_newer_keypad (UserInterface|GetWidget (Variables|Default|Getbutton_widget))))
  (EventDispatchers|BindEventtoOnClicked (Variables|/Game/Mikey/Blueprints/Widget_newer_keypad.Widget_newer_keypad_C|GetButton_1 _aswidget_newer_keypad) (delegate Custom|OnClicked_Button1))
  (EventDispatchers|AssignOnClicked (Variables|/Game/Mikey/Blueprints/Widget_newer_keypad.Widget_newer_keypad_C|GetButton_2 _aswidget_newer_keypad) (delegate Custom|OnClicked_Button2))
  (EventDispatchers|AssignOnClicked (Variables|/Game/Mikey/Blueprints/Widget_newer_keypad.Widget_newer_keypad_C|GetButton_3 _aswidget_newer_keypad) (delegate Custom|OnClicked_Button3))
  (EventDispatchers|AssignOnClicked (Variables|/Game/Mikey/Blueprints/Widget_newer_keypad.Widget_newer_keypad_C|GetButton_4 _aswidget_newer_keypad) (delegate Custom|OnClicked_Button4))
  (EventDispatchers|AssignOnClicked (Variables|/Game/Mikey/Blueprints/Widget_newer_keypad.Widget_newer_keypad_C|GetButton_5 _aswidget_newer_keypad) (delegate Custom|OnClicked_Button5))
  (EventDispatchers|AssignOnClicked (Variables|/Game/Mikey/Blueprints/Widget_newer_keypad.Widget_newer_keypad_C|GetButton_6 _aswidget_newer_keypad) (delegate Custom|OnClicked_Button6))
  (EventDispatchers|AssignOnClicked (Variables|/Game/Mikey/Blueprints/Widget_newer_keypad.Widget_newer_keypad_C|GetButton_7 _aswidget_newer_keypad) (delegate Custom|OnClicked_Button7))
  (EventDispatchers|AssignOnClicked (Variables|/Game/Mikey/Blueprints/Widget_newer_keypad.Widget_newer_keypad_C|GetButton_8 _aswidget_newer_keypad) (delegate Custom|OnClicked_Button8))
  (EventDispatchers|AssignOnClicked (Variables|/Game/Mikey/Blueprints/Widget_newer_keypad.Widget_newer_keypad_C|GetButton_9 _aswidget_newer_keypad) (delegate Custom|OnClicked_Button9))
  (EventDispatchers|AssignOnClicked (Variables|/Game/Mikey/Blueprints/Widget_newer_keypad.Widget_newer_keypad_C|GetButton_0 _aswidget_newer_keypad) (delegate Custom|OnClicked_Button0))
  (EventDispatchers|AssignOnClicked (Variables|/Game/Mikey/Blueprints/Widget_newer_keypad.Widget_newer_keypad_C|GetButton_back _aswidget_newer_keypad) (delegate Custom|OnClicked_ButtonBack))
  (EventDispatchers|AssignOnClicked (Variables|/Game/Mikey/Blueprints/Widget_newer_keypad.Widget_newer_keypad_C|GetButton_enter _aswidget_newer_keypad) (delegate Custom|OnClicked_ButtonEnter)))

(event Input|KeyboardEvents|E
  (params (Key :type Key%20Structure :default "None"))
  (:Pressed
    (CallFunction|ToggleCamera)))

(fn ConstructionScript)

(fn ToggleCamera
  (bind _returnvalue (Game|GetPlayerController 0))
  (bind _returnvalue_2 (Game|GetPlayerCharacter 0))
  (bind _output_get (Variables|Default|Setcamera_state (not (Variables|Default|Getcamera_state))))
  (if _output_get
    (Game|Player|SetViewTargetwithBlend _returnvalue (Components|GetOwner (Variables|Default|GetKeypad_camera)) 0.75 "VTBlend_Linear" 0.0 false)
    (Input|SetIgnoreMoveInput _returnvalue true)
    (Input|SetIgnoreLookInput _returnvalue true)
    (Variables|/Script/Engine.PlayerController|SetbShowMouseCursor _returnvalue true)
    (bind _asthird_person_character (Utilities|Casting|CastToThirdPersonCharacter _returnvalue_2))
    (Development|SetHiddeninGame (Variables|/Script/Engine.Character|GetMesh _asthird_person_character) true false)
    (else
      (Game|Player|SetViewTargetwithBlend _returnvalue _returnvalue_2 0.33 "VTBlend_Linear" 0.0 false)
      (Input|ResetIgnoreMoveInput _returnvalue)
      (Input|ResetIgnoreLookInput _returnvalue)
      (Variables|/Script/Engine.PlayerController|SetbShowMouseCursor _returnvalue false)
      (bind _asthird_person_character_2 (Utilities|Casting|CastToThirdPersonCharacter _returnvalue_2))
      (Development|SetHiddeninGame (Variables|/Script/Engine.Character|GetMesh _asthird_person_character_2) false false))))

(fn InitializeNumber
  (if (Variables|Default|Getnum1_init)
    (if (Variables|Default|Getnum2_init)
      (if (Variables|Default|Getnum3_init)
        (if (not (Variables|Default|Getnum4_init))
          (Variables|Default|Setnum4_init true))
        (else
          (Variables|Default|Setnum3_init true)))
      (else
        (Variables|Default|Setnum2_init true)))
    (else
      (Variables|Default|Setnum1_init true))))

(fn EnterNumber
  (params (num :type Integer))
  (if (Variables|Default|Getnum1_init)
    (if (Variables|Default|Getnum2_init)
      (if (Variables|Default|Getnum3_init)
        (if (not (Variables|Default|Getnum4_init))
          (Variables|Default|Setnum4 num))
        (else
          (Variables|Default|Setnum3 num)))
      (else
        (Variables|Default|Setnum2 num)))
    (else
      (Variables|Default|Setnum1 num))))