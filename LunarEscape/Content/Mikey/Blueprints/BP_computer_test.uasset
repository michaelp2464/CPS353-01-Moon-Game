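; Test interactable computer that switches the player from the third-person view to a computer camera.
; Overlap enables input for the E key, which calls ToggleCamera.
; ToggleCamera blends to the camera, locks move and look input, shows the cursor and hides the character mesh.
; It flips CameraState, but its branch condition is constant true, so the path restoring the player view never runs.
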(event Collision|EventActorBeginOverlap
  (params (OtherActor :type Actor%20Object%20Reference))
  (Utilities|Casting|CastToThirdPersonCharacter OtherActor)
  (Input|EnableInput (Game|GetPlayerController 0)))

(event Collision|EventActorEndOverlap
  (params (OtherActor :type Actor%20Object%20Reference))
  (Utilities|Casting|CastToThirdPersonCharacter OtherActor)
  (Input|DisableInput (Game|GetPlayerController 0)))

(event Input|KeyboardEvents|E
  (params (Key :type Key%20Structure :default "None"))
  (:Pressed
    (CallFunction|ToggleCamera)))

(fn ConstructionScript)

(fn ToggleCamera
  (bind _returnvalue (Game|GetPlayerController 0))
  (bind _returnvalue_2 (Game|GetPlayerCharacter 0))
  (Variables|Default|Setcamera_state (not (Variables|Default|Getcamera_state)))
  (if true
    (Game|Player|SetViewTargetwithBlend _returnvalue (Components|GetOwner (Variables|Default|Getcom_camera)) 0.75 "VTBlend_Linear" 0.0 false)
    (Input|SetIgnoreMoveInput _returnvalue true)
    (Input|SetIgnoreLookInput _returnvalue true)
    (Variables|/Script/Engine.PlayerController|SetbShowMouseCursor _returnvalue true)
    (bind _asthird_person_character (Utilities|Casting|CastToThirdPersonCharacter _returnvalue_2))
    (Development|SetHiddeninGame (Variables|/Script/Engine.Character|GetMesh _asthird_person_character) true false)
    (else
      (Game|Player|SetViewTargetwithBlend _returnvalue _returnvalue_2 0.33 "VTBlend_Linear" 0.0 false)
      (Input|ResetIgnoreMoveInput _returnvalue)
      (Input|ResetIgnoreLookInput _returnvalue)
      (Variables|/Script/Engine.PlayerController|SetbShowMouseCursor _returnvalue false)
      (bind _asthird_person_character_2 (Utilities|Casting|CastToThirdPersonCharacter _returnvalue_2))
      (Development|SetHiddeninGame (Variables|/Script/Engine.Character|GetMesh _asthird_person_character_2) false false))))