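; BP_New_Keypad is an interactable keypad actor that switches the player to a close-up camera view.
; Overlap with ThirdPersonCharacter enables its input, so pressing E calls ToggleKeycam, and leaving disables it.
; ToggleKeycam flips Camstate and blends the view target between the Keycam's owner and the player character, toggling move/look lock and mouse cursor.
; No button or code-entry logic is present in these graphs.
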(event Collision|EventActorEndOverlap
  (params (OtherActor :type Actor%20Object%20Reference))
  (Utilities|Casting|CastToThirdPersonCharacter OtherActor)
  (Input|DisableInput (Game|GetPlayerController 0)))

(event Collision|EventActorBeginOverlap
  (params (OtherActor :type Actor%20Object%20Reference))
  (Utilities|Casting|CastToThirdPersonCharacter OtherActor)
  (Input|EnableInput (Game|GetPlayerController 0)))

(event Input|KeyboardEvents|E
  (params (Key :type Key%20Structure :default "None"))
  (:Pressed
    (CallFunction|ToggleKeycam)))

(fn ConstructionScript)

(fn ToggleKeycam
  (bind _returnvalue (Game|GetPlayerController 0))
  (bind _output_get (Variables|Default|SetCamstate (not (Variables|Default|GetCamstate))))
  (if _output_get
    (Game|Player|SetViewTargetwithBlend _returnvalue (Components|GetOwner (Variables|Default|Getkeycam)) 0.75 "VTBlend_Linear" 0.0 false)
    (Input|SetIgnoreMoveInput _returnvalue true)
    (Input|SetIgnoreLookInput _returnvalue true)
    (Variables|/Script/Engine.PlayerController|SetbShowMouseCursor _returnvalue true)
    (else
      (Game|Player|SetViewTargetwithBlend _returnvalue (Game|GetPlayerCharacter 0) 0.33 "VTBlend_Linear" 0.0 false)
      (Input|ResetIgnoreMoveInput _returnvalue)
      (Input|ResetIgnoreLookInput _returnvalue)
      (Variables|/Script/Engine.PlayerController|SetbShowMouseCursor _returnvalue false))))