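; Fuse box lever that the player pulls with E while overlapping it, switching the power for the level's lights.
; Overlap with ThirdPersonCharacter enables or disables input; a press plays a sound and a Timeline rotating the lever.
; After an eight-second delay it flips IsOn and calls switch functions on every BP_Spotlight, BP_Pointlight and BP_BasementLamp.
; No guard enforces the one-time use noted in the comments.
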(event Collision|EventActorBeginOverlap
  (params (OtherActor :type Actor%20Object%20Reference))
  ;[1 1 1] Enable/Disable -JOSHUA
  (Utilities|Casting|CastToThirdPersonCharacter OtherActor)
  (Input|EnableInput (Game|GetPlayerController 0)))

(event Collision|EventActorEndOverlap
  (params (OtherActor :type Actor%20Object%20Reference))
  ;[1 1 1] Enable/Disable -JOSHUA
  (Utilities|Casting|CastToThirdPersonCharacter OtherActor)
  (Input|DisableInput (Game|GetPlayerController 0)))

(event Input|KeyboardEvents|E
  (params (Key :type Key%20Structure :default "None"))
  (:Pressed
    (Utilities|FlowControl|Sequence
      (:then_0
        (Audio|PlaySound2D "/Game/Joshua/Sounds/TurningOnPower_Sound/Turning_on_the_Power.Turning_on_the_Power" 1.0 1.0 0.0 0 0)
        (Utilities|FlowControl|Delay 8.0)
        ;[1 1 1] Lights set to OFF-JOSHUA
        (Variables|Default|SetisOn (not (Variables|Default|GetisOn)))
        (Utilities|FlowControl|Sequence
          (:then_0
            ;[1 1 1] Array to turn on all spotlights-JOSHUA
            (bind _outactors (Actor|GetAllActorsOfClass "/Game/Joshua/BluePrints/BP_Spotlight.BP_Spotlight_C"))
            (for _array_element _outactors
              (Default|LightSwitch _array_element)))
          (:then_1
            ;[1 1 1] Array to turn on all pointlights-JOSHUA
            (bind _outactors_2 (Actor|GetAllActorsOfClass "/Game/Joshua/BluePrints/BP_Pointlight.BP_Pointlight_C"))
            (for _array_element_2 _outactors_2
              (Default|LightSwitch2 _array_element_2)))
          (:then_2
            ;[1 1 1] Array to make the lamps glow-JOSHUA
            (bind _outactors_3 (Actor|GetAllActorsOfClass "/Game/Joshua/BluePrints/BP_BasementLamp.BP_BasementLamp_C"))
            (for _array_element_3 _outactors_3
              (Default|GlowSwitch _array_element_3)))))
      (:then_1
        ;[1 1 1] Animation-JOSHUA
        (bind _newtrack_0 (Timeline|Timeline_0 Play)
          (:Update
            (Transformation|SetRelativeLocationAndRotation (Variables|Default|GetStaticMeshComponent1) "0, 0, 0" (Math|Rotator|Lerp(Rotator) "0, 0, 0" "-40.000000,0.000000, 0" _newtrack_0) false false)))))))

(fn ConstructionScript)