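; BP_HazardLight is a hazard alarm light with rotating movement and audio.
; After BeginPlay, it waits a fixed delay, then fades in the alarm sound.
; StopAlarm halts rotation by clearing the movement's updated component and hides the Left and Right components.
; It also swaps both light meshes to gray and stops audio, but only if Actor4 casts to BP_FuseBoxLever.
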(event EventBeginPlay
  (Utilities|FlowControl|Delay 73.0)
  (Audio|Components|Audio|FadeIn (Variables|Default|GetAudio) 3.0 1.0 0.0 "Linear" :!class /Script/Engine.AudioComponent))

(fn ConstructionScript)

(fn StopAlarm
  (Utilities|FlowControl|Sequence
    (:then_0
      (Components|Movement|SetUpdatedComponent (Variables|Default|GetRotatingMovement) 0)
      (Components|Movement|StopMovementImmediately (Variables|Default|GetRotatingMovement)))
    (:then_1
      (Utilities|Casting|CastToBP_FuseBoxLever (Variables|Default|GetActor%204))
      (Rendering|Material|SetMaterial (Variables|Default|GetLight1) 0 "/Game/StarterBundle/ModularSci_Comm/Materials/MI_Ceiling_OuterRing_BC_Gray.MI_Ceiling_OuterRing_BC_Gray")
      (Rendering|Material|SetMaterial (Variables|Default|GetLight2) 0 "/Game/StarterBundle/ModularSci_Comm/Materials/MI_Ceiling_OuterRing_BC_Gray.MI_Ceiling_OuterRing_BC_Gray")
      (Audio|Components|Audio|Stop (Variables|Default|GetAudio)))
    (:then_2
      (Rendering|SetVisibility (Variables|Default|GetLeft) false false)
      (Rendering|SetVisibility (Variables|Default|GetRight) false false))))