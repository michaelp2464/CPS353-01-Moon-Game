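; Interactable spacesuit actor that the player puts on with E while overlapping it, gated by whether the referenced cube holder has its cube inserted.
; Overlap toggles input on the actor.
; Pressing E forces and locks first-person view, hides the suit and disables its collision, then covers the screen with a black widget and zipper sound.
; After a short delay it shows a helmet border, disables the character HUD and flags the suit as on.
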(event Collision|EventActorBeginOverlap
  (params (OtherActor :type Actor%20Object%20Reference))
  ;[1 1 1] -Rob
  ;;[1 1 1] Enable/Disable input on overlap
  (Input|EnableInput (Game|GetPlayerController 0)))

(event Collision|EventActorEndOverlap
  (params (OtherActor :type Actor%20Object%20Reference))
  ;[1 1 1] -Rob
  ;;[1 1 1] Enable/Disable input on overlap
  (Input|DisableInput (Game|GetPlayerController 0)))

(event Input|KeyboardEvents|E
  (params (Key :type Key%20Structure :default "None"))
  (bind _returnvalue (Game|GetPlayerController 0))
  ;[1 1 1] -Rob
  ;;[1 1 1] "Putting on suit" sequence
  (:Pressed
    (Variables|Default|SetcanExitWithSuit (Variables|/Game/Rob/Blueprints/WindowPostCubeHolder.WindowPostCubeHolder_C|GetcubeIn (Variables|Default|GetCUBEHOLDER)))
    (if (Variables|Default|GetcanExitWithSuit)
      (bind _asthird_person_character (Utilities|Casting|CastToThirdPersonCharacter (Game|GetPlayerCharacter 0)))
      (if (Variables|/Game/ThirdPersonBP/Blueprints/ThirdPersonCharacter.ThirdPersonCharacter_C|GetisThirdPerson _asthird_person_character)
        (Default|ToggleThirdPerson _asthird_person_character))
      (Variables|/Game/ThirdPersonBP/Blueprints/ThirdPersonCharacter.ThirdPersonCharacter_C|SetthirdPersonLocked _asthird_person_character true)
      (bind _returnvalue_2 (UserInterface|CreateWidget "/Game/Rob/Widgets/HelmetBorder.HelmetBorder_C" _returnvalue))
      (bind _returnvalue_3 (UserInterface|CreateWidget "/Game/Rob/Widgets/TempBlackScreen.TempBlackScreen_C" _returnvalue))
      (Collision|SetActorEnableCollision false)
      (Rendering|SetVisibility (Variables|SkeletalMeshActor|GetSkeletalMeshComponent) false false)
      (UserInterface|Viewport|AddtoViewport _returnvalue_3 0)
      (Audio|PlaySoundatLocation "/Game/Rob/UsedSounds/zippersound.zippersound" "0, 0, 0" "0, 0, 0" 0.2 0.9 0.2 0 0 0)
      (Utilities|FlowControl|Delay 1.5)
      (Widget|SetVisibility _returnvalue_3 "Collapsed")
      (UserInterface|Viewport|AddtoViewport _returnvalue_2 0)
      (bind _asthird_person_character_2 (Utilities|Casting|CastToThirdPersonCharacter (Game|GetPlayerCharacter 0)))
      (Default|DisableHUD _asthird_person_character_2 true)
      (Variables|Default|SetsuitIsOn true))))

(fn ConstructionScript)