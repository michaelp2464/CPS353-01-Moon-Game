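; A locked sliding station door that signals it cannot be opened with an alarm sound and flashing lights.
; Overlapping the actor enables player input on it, and leaving disables it.
; Pressing E plays the alarm at the door's location from partway into the clip and briefly brightens four point lights before dimming them again.
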(event Collision|EventActorBeginOverlap
  (params (OtherActor :type Actor%20Object%20Reference))
  ;[1 1 1] Quick locked door, lights flash, plays alarm noise -Rob
  (Input|EnableInput (Game|GetPlayerController 0)))

(event Collision|EventActorEndOverlap
  (params (OtherActor :type Actor%20Object%20Reference))
  ;[1 1 1] Quick locked door, lights flash, plays alarm noise -Rob
  (Input|DisableInput (Game|GetPlayerController 0)))

(event Input|KeyboardEvents|E
  (params (Key :type Key%20Structure :default "None"))
  (bind _pointlight (Variables|Default|GetPointLight))
  ;[1 1 1] Quick locked door, lights flash, plays alarm noise -Rob
  (:Pressed
    (Audio|PlaySoundatLocation "/Game/Rob/UsedSounds/AlarmDoor.AlarmDoor" (Transformation|GetWorldLocation (Variables|Default|GetStationDoor)) "0, 0, 0" 1.0 1.0 1e+01 0 0 0)
    (Rendering|Components|Light|SetIntensity _pointlight 5e+03)
    (Utilities|FlowControl|Delay 0.2)
    (Rendering|Components|Light|SetIntensity _pointlight 1e+03)))

(fn ConstructionScript)