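; Final station door that starts its ending sequence when the player presses E in its overlap area, with the cube puzzle solved and suit on.
; Otherwise it sounds an alarm, except while an unsolved cube is inserted.
; Four point lights blink constantly via a delay loop from BeginPlay.
; The ending turns them red, plays sounds, moves the opposite door while the player character watches, then slides this door up after a delay.
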(event Custom|endingCondition
  (bind _oppositedoor (Variables|Default|GetOPPOSITEDOOR))
  ;[1 1 1] Sequence for unlocking the final door -Rob
  (Utilities|FlowControl|Sequence
    (:then_0
      (Audio|PlaySoundatLocation "/Engine/VREditor/Sounds/VR_open_Cue.VR_open_Cue" "0, 0, 0" "0, 0, 0" 1.0 1.0 0.0 0 0 0)
      (Rendering|Components|Light|SetLightColor (Variables|Default|GetPointLight1) "(R=1.000000,G=0.000000,B=0.013170,A=1.000000)" true)
      (Utilities|FlowControl|Delay 1.0)
      (Audio|PlaySoundatLocation "/Game/Rob/UsedSounds/Alarmslow.Alarmslow" (Transformation|GetWorldLocation (Variables|Default|GetStationDoor)) "0, 0, 0" 0.5 0.5 0.0 "/Game/Joshua/Sounds/Slidingdoor_Sounds/SlidingDoorAttenuation.SlidingDoorAttenuation" 0 0)
      (Utilities|FlowControl|Delay 1.0))
    (:then_1
      (bind _asthird_person_character (Utilities|Casting|CastToThirdPersonCharacter (Game|GetPlayerCharacter 0)))
      (bind _newtrack_0 (Timeline|Timeline_1 PlayFromStart)
        (:Update
          (Default|WatchObject _asthird_person_character _oppositedoor)
          (Transformation|SetWorldLocation (Variables|/Script/Engine.Actor|GetRootComponent (Variables|Default|GetOPPOSITEDOOR)) (Math|Vector|Lerp(Vector) (Variables|/Script/Engine.SceneComponent|GetRelativeLocation (Variables|/Script/Engine.Actor|GetRootComponent _oppositedoor)) (Math|Vector|MakeVector 2034.0 912.0 201.0) _newtrack_0) false false))))
    (:then_2
      (Utilities|FlowControl|Delay 5.0)
      (bind _newtrack_0_2 (Timeline|Timeline_0 PlayFromStart)
        (:Update
          (Transformation|SetRelativeLocation (Variables|Default|GetStationDoor) (Math|Vector|Lerp(Vector) "0, 0, 0" "0.000000, 0,400.000000" _newtrack_0_2) false false))))))

(event EventBeginPlay
  (bind _pointlight (Variables|Default|GetPointLight))
  ;[1 1 1] Lights Blink at all times -Rob
  (Rendering|Components|Light|SetIntensity _pointlight 5e+03 :!label _label)
  (Utilities|FlowControl|Delay 0.2)
  (Rendering|Components|Light|SetIntensity _pointlight 1e+03)
  (Utilities|FlowControl|Delay 0.2)
  (goto _label))

(event Collision|EventActorBeginOverlap
  (params (OtherActor :type Actor%20Object%20Reference))
  ;[1 1 1] Quick locked door, lights flash, plays alarm noise -Rob
  (Input|EnableInput (Game|GetPlayerController 0)))

(event Collision|EventActorEndOverlap
  (params (OtherActor :type Actor%20Object%20Reference))
  ;[1 1 1] Quick locked door, lights flash, plays alarm noise -Rob
  (Input|DisableInput (Game|GetPlayerController 0)))

(event Input|KeyboardEvents|E
  (params (Key :type Key%20Structure :default "None"))
  (bind _cubeholder (Variables|Default|GetCUBEHOLDER))
  ;[1 1 1] Quick locked door, lights flash, plays alarm noise -Rob
  (:Pressed
    (if (and (Variables|/Game/Rob/Blueprints/WindowPostCubeHolder.WindowPostCubeHolder_C|GetisSolved (Variables|Default|GetCUBEHOLDER)) (Variables|/Game/Rob/Blueprints/Spacesuit_Blueprint.Spacesuit_Blueprint_C|GetsuitIsOn (Variables|Default|GetSUIT)))
      (CallFunction|EndingCondition)
      (elif (not (and (Variables|/Game/Rob/Blueprints/WindowPostCubeHolder.WindowPostCubeHolder_C|GetcubeIn _cubeholder) (not (Variables|/Game/Rob/Blueprints/WindowPostCubeHolder.WindowPostCubeHolder_C|GetisSolved _cubeholder))))
        (Audio|PlaySoundatLocation "/Game/Rob/UsedSounds/AlarmDoor.AlarmDoor" (Transformation|GetWorldLocation (Variables|Default|GetStationDoor)) "0, 0, 0" 1.0 1.0 1e+01 0 0 0)))))

(fn ConstructionScript)