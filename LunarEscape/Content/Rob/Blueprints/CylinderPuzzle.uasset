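; Timed cylinder puzzle that the player operates with E when nearby, provided its cube holder is filled.
; E toggles a puzzle camera, hiding the character and showing clickable arrows that shift the outer cylinder between three positions.
; A looping timer rotates the inner cylinder and, on alternating ticks, checks that position against a per-tick answer array.
; A streak of correct checks fires SolvedEvent, while a miss resets the count.
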(event OnClicked(rightButton)
  (params (TouchedComponent :type Primitive%20Component%20Object%20Reference) (ButtonPressed :type Key%20Structure :default "None"))
  ;[1 1 1] Puzzle solving mode -Rob
  (switch int (Variables|Default|GetcurrentPosition)
    (:0
      (Transformation|SetWorldLocation (Variables|Default|GetOuterCylinder) (Variables|Default|GetOuterCylinderLocCenter) false false)
      (Variables|Default|SetcurrentPosition 1))
    (:1
      (Transformation|SetWorldLocation (Variables|Default|GetOuterCylinder) (Variables|Default|GetOuterCylinderLocRight) false false)
      (Variables|Default|SetcurrentPosition 2))))

(event OnClicked(leftButton)
  (params (TouchedComponent :type Primitive%20Component%20Object%20Reference) (ButtonPressed :type Key%20Structure :default "None"))
  ;[1 1 1] Puzzle solving mode -Rob
  (switch int (Variables|Default|GetcurrentPosition)
    (:1
      (Transformation|SetWorldLocation (Variables|Default|GetOuterCylinder) (Variables|Default|GetOuterCylinderLocLeft) false false)
      (Variables|Default|SetcurrentPosition 0))
    (:2
      (Transformation|SetWorldLocation (Variables|Default|GetOuterCylinder) (Variables|Default|GetOuterCylinderLocCenter) false false)
      (Variables|Default|SetcurrentPosition 1))))

(event Custom|PuzzleTick
  ;[1 1 1] Puzzle solving mode -Rob
  (Utilities|FlowControl|FlipFlop
    (:A
      _)
    (:B
      (if (== (Variables|Default|GettickNum) 2)
        _
        (else
          (CallFunction|CheckifCorrectPos)))))
  (Transformation|AddWorldRotation (Variables|Default|GetInnerCylinder) (Math|Rotator|MakeRotator 0.0 22.5 0.0) false false)
  (if (== (Variables|Default|GettickNum) 15)
    (Variables|Default|SettickNum 0)
    (else
      (bind _result (Math|Integer|IncrementInt (Variables|Default|GettickNum))
        (:%20%20
          (Variables|Default|SettickNum _result))))))

(event Custom|Toggle%20Camera
  (bind _returnvalue (Game|GetPlayerController 0))
  (bind _returnvalue_2 (Game|GetPlayerCharacter 0))
  ;[1 1 1] Code taken from Ben's trash bin BP
  ;;[1 1 1] Tell the HUD in ThirdPersonCharacter to disable
  (bind _asthird_person_character (Utilities|Casting|CastToThirdPersonCharacter (Game|GetPlayerCharacter 0)))
  (Default|DisableHUD _asthird_person_character (not (Variables|Default|GetCamera%20State)))
  (bind _output_get (Variables|Default|SetCamera%20State (not (Variables|Default|GetCamera%20State))))
  (if _output_get
    (Game|Player|SetViewTargetwithBlend _returnvalue (Components|GetOwner (Actor|GetComponentbyClass self "/Script/Engine.ActorComponent")) 0.75 "VTBlend_Linear" 0.0 false)
    (Input|SetIgnoreMoveInput _returnvalue true)
    (Input|SetIgnoreLookInput _returnvalue true)
    (bind _asthird_person_character_2 (Utilities|Casting|CastToThirdPersonCharacter _returnvalue_2))
    (Development|SetHiddeninGame (Variables|/Script/Engine.Character|GetMesh _asthird_person_character_2) true false)
    (else
      (Game|Player|SetViewTargetwithBlend _returnvalue _returnvalue_2 0.33 "VTBlend_Linear" 0.0 false)
      (Input|ResetIgnoreMoveInput _returnvalue)
      (Input|ResetIgnoreLookInput _returnvalue)
      (bind _asthird_person_character_3 (Utilities|Casting|CastToThirdPersonCharacter _returnvalue_2))
      (Development|SetHiddeninGame (Variables|/Script/Engine.Character|GetMesh _asthird_person_character_3) false false))))

(event Custom|Solve%20Mode
  ;[1 1 1] Puzzle solving mode -Rob
  (Utilities|FlowControl|Sequence
    (:then_0
      (Variables|/Script/Engine.PlayerController|SetbEnableClickEvents (Game|GetPlayerController 0) true)
      (CallFunction|GetLocations)
      (CallFunction|FlipArrowVisibility))
    (:then_1
      (Utilities|Time|SetTimerbyEvent (delegate Custom|PuzzleTick) 1.5 (Variables|Default|GetinSolveMode)))))

(event Collision|EventActorBeginOverlap
  (params (OtherActor :type Actor%20Object%20Reference))
  ;[1 1 1] Enable/disable input when nearby
  (if (Variables|/Game/Rob/Blueprints/WindowPostCubeHolder.WindowPostCubeHolder_C|GetcubeIn (Variables|Default|GetCUBEHOLDER))
    (Input|EnableInput (Game|GetPlayerController 0))))

(event Collision|EventActorEndOverlap
  (params (OtherActor :type Actor%20Object%20Reference))
  ;[1 1 1] Enable/disable input when nearby
  (Input|DisableInput (Game|GetPlayerController 0)))

(event Input|KeyboardEvents|E
  (params (Key :type Key%20Structure :default "None"))
  (bind _returnvalue (Game|GetPlayerController 0))
  ;[1 1 1] Code taken from Ben's trash bin BP
  (:Pressed
    (CallFunction|ToggleCamera)
    (if (Variables|Default|GetCamera%20State)
      (Variables|/Script/Engine.PlayerController|SetbShowMouseCursor _returnvalue true)
      ;;[1 1 1] Rob added code
      (Variables|Default|SetinSolveMode true)
      (CallFunction|SolveMode)
      (else
        (Variables|/Script/Engine.PlayerController|SetbShowMouseCursor _returnvalue false)
        (Variables|/Script/Engine.PlayerController|SetbEnableClickEvents (Game|GetPlayerController 0) false)
        (Variables|Default|SetinSolveMode false)
        (CallFunction|FlipArrowVisibility)))))

(fn ConstructionScript)

(fn GetLocations
  (Variables|Default|SetOuterCylinderLocCenter (Transformation|GetWorldLocation (Variables|Default|GetOuterCylinder)))
  (Variables|Default|SetOuterCylinderLocLeft (Math|Vector|MakeVector (.X (Math|Vector|BreakVector (Variables|Default|GetOuterCylinderLocCenter))) (+ (.Y (Math|Vector|BreakVector (Variables|Default|GetOuterCylinderLocCenter))) -4.5) (.Z (Math|Vector|BreakVector (Variables|Default|GetOuterCylinderLocCenter)))))
  (Variables|Default|SetOuterCylinderLocRight (Math|Vector|MakeVector (.X (Math|Vector|BreakVector (Variables|Default|GetOuterCylinderLocCenter))) (+ (.Y (Math|Vector|BreakVector (Variables|Default|GetOuterCylinderLocCenter))) 4.5) (.Z (Math|Vector|BreakVector (Variables|Default|GetOuterCylinderLocCenter))))))

(fn CheckifCorrectPos
  (bind _defaultsceneroot (Variables|Default|GetDefaultSceneRoot))
  (bind _returnvalue (Transformation|GetWorldLocation _defaultsceneroot))
  (if (== (Variables|Default|GetcurrentPosition) (Utilities|Array|Get(acopy) (Variables|Default|GetcorrectLocsByTick) (Variables|Default|GettickNum)))
    (bind _result (Math|Integer|IncrementInt (Variables|Default|GetcorrectCount))
      (:%20%20
        (if (== _result 7)
          (Audio|PlaySoundatLocation "/Game/Ben/B_Sounds/puzzle_success.puzzle_success" _returnvalue "0, 0, 0" 1.0 1.0 0.0 0 0 0)
          (Variables|Default|SetisSolved true)
          (Variables|Default|SetinSolveMode false)
          (Development|PrintString "Done")
          (CallFunction|SolvedEvent)
          (else
            (Audio|PlaySoundatLocation "/Game/BranMan/12-2-2022Push/BranMan/GunSounds/SuccessSound.SuccessSound" _returnvalue "0, 0, 0" 1.0 1.0 0.0 0 0 0)
            (Development|PrintString "Correct not there yet")))))
    (else
      (Variables|Default|SetcorrectCount 0)
      (Audio|PlaySoundatLocation "/Engine/VREditor/Sounds/UI/Invalid_Action.Invalid_Action" _returnvalue "0, 0, 0" 1.0 1.0 0.0 0 0 0)
      (Development|PrintString "Bad bad bad"))))

(fn FlipArrowVisibility
  (Rendering|SetVisibility (Variables|Default|GetleftButton) (not (Variables|Default|GetvisibleButtons)) false)
  (Variables|Default|SetvisibleButtons (not (Variables|Default|GetvisibleButtons))))