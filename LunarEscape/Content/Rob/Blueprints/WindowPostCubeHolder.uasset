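; A wall post that accepts the Rubik's cube: pressing E while the cube overlaps it locks the cube into its slot, once only.
; Overlap with BP_RubiksCube toggles player input on the actor.
; E stops the cube's tick, snaps it to the slot and slides it in via timeline, then lowers the panel door with a closing sound.
; A delayed sequence then plays rising sounds and reveals three point lights one by one.
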(event Custom|ClosePanel
  (bind _panel (Variables|Default|GetPanel))
  (bind _returnvalue (Transformation|GetWorldLocation _panel))
  (bind (_x _y _z) (Math|Vector|BreakVector _returnvalue))
  ;[1 1 1] Closes Panel Door - Rob
  (bind _newtrack_0 (Timeline|Timeline_0 Play)
    (:Update
      (Transformation|SetWorldLocation (Variables|Default|GetPanel) (Math|Vector|Lerp(Vector) _returnvalue (Math|Vector|MakeVector _x _y (- _z 2.0)) _newtrack_0) false false))
    (:Finished
      (Audio|PlaySoundatLocation "/Game/Rob/UsedSounds/PanelClose.PanelClose" _returnvalue "0, 0, 0" 2.0 1.0 0.0 0 0 0))))

(event Custom|MoveCubeIn
  (bind _cubeslot (Variables|Default|GetCubeSlot))
  (bind _returnvalue (Transformation|GetWorldLocation _cubeslot))
  (bind (_x _y _z) (Math|Vector|BreakVector _returnvalue))
  ;[1 1 1] Move cube into slot -Rob
  (bind _newtrack_0 (Timeline|Timeline_1 PlayFromStart)
    (:Update
      (Transformation|SetWorldLocation (Variables|/Script/Engine.Actor|GetRootComponent (Variables|Default|GetCUBE)) (Math|Vector|Lerp(Vector) (Transformation|GetWorldLocation (Variables|Default|GetCubeSlot)) (Math|Vector|MakeVector (+ _x 55.0) _y _z) _newtrack_0) false false))))

(event Custom|Teleport%20Cube
  (bind _cube (Variables|Default|GetCUBE))
  (bind _rootcomponent (Variables|/Script/Engine.Actor|GetRootComponent _cube))
  ;[1 1 1] Teleports cube in front of slot
  (Actor|Tick|SetActorTickEnabled _cube)
  (Transformation|SetWorldRotation _rootcomponent "0, 0, 0" false false)
  (Transformation|SetWorldLocation _rootcomponent (Transformation|GetWorldLocation (Variables|Default|GetCubeSlot)) false false))

(event Custom|LightOnSequence
  (bind _staticmesh (Variables|Default|GetStaticMesh))
  (bind _returnvalue (Transformation|GetWorldLocation _staticmesh))
  (Utilities|FlowControl|Sequence
    (:then_0
      (Utilities|FlowControl|Delay 1.8)
      (Audio|PlaySoundatLocation "/Game/Rob/UsedSounds/ScaleUp1.ScaleUp1" _returnvalue "0, 0, 0" 1.0 1.0 0.0 0 0 0)
      (Utilities|FlowControl|Delay 2.2)
      (Audio|PlaySoundatLocation "/Game/Rob/UsedSounds/Scaleup2.Scaleup2" _returnvalue "0, 0, 0" 1.0 1.0 0.0 0 0 0))
    (:then_1
      (Utilities|FlowControl|Delay 3.0)
      (Rendering|SetVisibility (Variables|Default|GetPointLight1) true false)
      (Utilities|FlowControl|Delay 1.0)
      (Rendering|SetVisibility (Variables|Default|GetPointLight2) true false)
      (Utilities|FlowControl|Delay 1.0)
      (Rendering|SetVisibility (Variables|Default|GetPointLight3) true false))))

(event Collision|EventActorBeginOverlap
  (params (OtherActor :type Actor%20Object%20Reference))
  ;[1 1 1] Enable Input if Cube in Position
  (if (== (Utilities|GetClass OtherActor) "/Game/Rob/Blueprints/BP_RubiksCube.BP_RubiksCube_C")
    (Input|EnableInput (Game|GetPlayerController 0))))

(event Collision|EventActorEndOverlap
  (params (OtherActor :type Actor%20Object%20Reference))
  ;[1 1 1] Disable input after leaving -Rob
  (if (== (Utilities|GetClass OtherActor) "/Game/Rob/Blueprints/BP_RubiksCube.BP_RubiksCube_C")
    (Input|DisableInput (Game|GetPlayerController 0))))

(event Input|KeyboardEvents|E
  (params (Key :type Key%20Structure :default "None"))
  ;[1 1 1] Sequence for entering cube
  (:Pressed
    (if (not (Variables|Default|GetcubeIn))
      (Utilities|FlowControl|Sequence
        (:then_0
          (Variables|Default|SetcubeIn true))
        (:then_1
          (CallFunction|TeleportCube))
        (:then_2
          (CallFunction|MoveCubein))
        (:then_3
          (Utilities|FlowControl|Delay 1.0)
          (CallFunction|ClosePanel))
        (:then_4
          (CallFunction|LightonSequence))))))

(fn ConstructionScript)