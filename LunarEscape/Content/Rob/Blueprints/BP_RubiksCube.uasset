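; BP_RubiksCube is an interactive 2x2 Rubik's cube puzzle, scrambled at BeginPlay from a list of face turns.
; Solve mode raises it to camera height, locks the player, and enables mouse-drag rotation and face buttons.
; FaceRot turns four cubes and updates per-face membership arrays, which IsWin compares to the starting layout.
; Winning exits solve mode and lights up; a gated Equip input gives an item when IsSolved is true.
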(event OnComponentEndOverlap(BoxCollision)
  (params (OverlappedComponent :type Primitive%20Component%20Object%20Reference) (OtherActor :type Actor%20Object%20Reference) (OtherComp :type Primitive%20Component%20Object%20Reference) (OtherBodyIndex :type Integer))
  ;[1 1 1] Everything I changed is in this box -Ben
  (Utilities|Casting|CastToThirdPersonCharacter OtherActor)
  (Input|DisableInput (Game|GetPlayerController 0))
  (Utilities|FlowControl|Gate true) ; enters at Close
)

(event OnComponentBeginOverlap(BoxCollision)
  (params (OverlappedComponent :type Primitive%20Component%20Object%20Reference) (OtherActor :type Actor%20Object%20Reference) (OtherComp :type Primitive%20Component%20Object%20Reference) (OtherBodyIndex :type Integer) (bFromSweep :type Boolean) (SweepResult :type Hit%20Result%20Structure%20%28by%20ref%29))
  ;[1 1 1] Everything I changed is in this box -Ben
  (Utilities|Casting|CastToThirdPersonCharacter OtherActor)
  (Input|EnableInput (Game|GetPlayerController 0))
  (Utilities|FlowControl|Gate true) ; enters at Open
)

(event OnClicked(ButtonE)
  (params (TouchedComponent :type Primitive%20Component%20Object%20Reference) (ButtonPressed :type Key%20Structure :default "None"))
  ;[1 1 1] On button click -> call for face rotation -Rob
  (Audio|PlaySoundatLocation "/Game/Mikey/Sounds/button_sound.button_sound" (Transformation|GetWorldLocation (Variables|Default|GetCubeCenter)) "0, 0, 0" 1.0 1.0 0.0 0 0 0)
  (CallFunction|FaceRot "E")
  (CallFunction|IsWin))

(event OnClicked(ButtonF)
  (params (TouchedComponent :type Primitive%20Component%20Object%20Reference) (ButtonPressed :type Key%20Structure :default "None"))
  ;[1 1 1] On button click -> call for face rotation -Rob
  (Audio|PlaySoundatLocation "/Game/Mikey/Sounds/button_sound.button_sound" (Transformation|GetWorldLocation (Variables|Default|GetCubeCenter)) "0, 0, 0" 1.0 1.0 0.0 0 0 0)
  (CallFunction|FaceRot "F")
  (CallFunction|IsWin))

(event OnClicked(ButtonA)
  (params (TouchedComponent :type Primitive%20Component%20Object%20Reference) (ButtonPressed :type Key%20Structure :default "None"))
  ;[1 1 1] On button click -> call for face rotation -Rob
  (Audio|PlaySoundatLocation "/Game/Mikey/Sounds/button_sound.button_sound" (Transformation|GetWorldLocation (Variables|Default|GetCubeCenter)) "0, 0, 0" 1.0 1.0 0.0 0 0 0)
  (CallFunction|FaceRot "A")
  (CallFunction|IsWin))

(event OnClicked(ButtonB)
  (params (TouchedComponent :type Primitive%20Component%20Object%20Reference) (ButtonPressed :type Key%20Structure :default "None"))
  ;[1 1 1] On button click -> call for face rotation -Rob
  (Audio|PlaySoundatLocation "/Game/Mikey/Sounds/button_sound.button_sound" (Transformation|GetWorldLocation (Variables|Default|GetCubeCenter)) "0, 0, 0" 1.0 1.0 0.0 0 0 0)
  (CallFunction|FaceRot "B")
  (CallFunction|IsWin))

(event OnClicked(ButtonC)
  (params (TouchedComponent :type Primitive%20Component%20Object%20Reference) (ButtonPressed :type Key%20Structure :default "None"))
  ;[1 1 1] On button click -> call for face rotation -Rob
  (Audio|PlaySoundatLocation "/Game/Mikey/Sounds/button_sound.button_sound" (Transformation|GetWorldLocation (Variables|Default|GetCubeCenter)) "0, 0, 0" 1.0 1.0 0.0 0 0 0)
  (CallFunction|FaceRot "C")
  (CallFunction|IsWin))

(event OnClicked(ButtonD)
  (params (TouchedComponent :type Primitive%20Component%20Object%20Reference) (ButtonPressed :type Key%20Structure :default "None"))
  ;[1 1 1] On button click -> call for face rotation -Rob
  (Audio|PlaySoundatLocation "/Game/Mikey/Sounds/button_sound.button_sound" (Transformation|GetWorldLocation (Variables|Default|GetCubeCenter)) "0, 0, 0" 1.0 1.0 0.0 0 0 0)
  (CallFunction|FaceRot "D")
  (CallFunction|IsWin))

(event Custom|setSolveModeOff
  (bind _returnvalue (Game|GetPlayerController 0))
  (bind _returnvalue_2 (Game|GetPlayerController 0))
  ;[1 1 1] Sets character back to normal to leave puzzle-solving position -Rob
  (CallFunction|ToggleButtonVisibility)
  (Input|ResetIgnoreLookInput _returnvalue)
  (Input|ResetIgnoreMoveInput _returnvalue)
  (Variables|/Script/Engine.PlayerController|SetbShowMouseCursor _returnvalue false)
  (Input|DisableInput _returnvalue_2)
  (Variables|/Script/Engine.PlayerController|SetbEnableClickEvents _returnvalue_2 false)
  (Variables|Default|SetisInCubeSolveMode false)
  (bind _asthird_person_character (Utilities|Casting|CastToThirdPersonCharacter (Game|GetPlayerCharacter 0)))
  (Default|DisableHUD _asthird_person_character false))

(event Custom|solveMode
  ;[1 1 1] Mode to rotate and edit cube -Rob
  (Variables|/Script/Engine.PlayerController|SetbEnableClickEvents (Game|GetPlayerController 0) true)
  (Utilities|Time|SetTimerbyEvent (delegate Custom|checkForMovement) 0.01 (Variables|Default|GetisInCubeSolveMode)))

(event Custom|setSolveModeOn
  (bind _returnvalue (Game|GetPlayerController 0))
  (bind _defaultsceneroot (Variables|Default|GetDefaultSceneRoot))
  (bind _returnvalue_2 (Transformation|GetWorldLocation _defaultsceneroot))
  (bind (_x _y) (Math|Vector|BreakVector _returnvalue_2))
  ;[1 1 1] Sets up camera and Rubiks cube position to solve the puzzle -Rob
  (Input|EnableInput (Game|GetPlayerController 0))
  (CallFunction|ToggleButtonVisibility)
  (bind _newtrack (Timeline|Timeline_0 PlayFromStart)
    (:Update
      (Transformation|SetWorldLocation (Variables|Default|GetDefaultSceneRoot) (Math|Vector|Lerp(Vector) _returnvalue_2 (Math|Vector|MakeVector _x _y (.Z (Math|Vector|BreakVector (Camera|GetCameraLocation (Game|GetPlayerCameraManager 0))))) _newtrack) false false)
      (bind _asthird_person_character (Utilities|Casting|CastToThirdPersonCharacter (Game|GetPlayerCharacter 0)))
      (Default|WatchObject _asthird_person_character self))
    (:Finished
      (Input|SetIgnoreMoveInput _returnvalue true)
      (Input|SetIgnoreLookInput _returnvalue true)
      (Variables|/Script/Engine.PlayerController|SetbShowMouseCursor _returnvalue true)
      (Variables|Default|SetisInCubeSolveMode true)
      (bind _asthird_person_character_2 (Utilities|Casting|CastToThirdPersonCharacter (Game|GetPlayerCharacter 0)))
      (Default|DisableHUD _asthird_person_character_2 true)
      (CallFunction|SolveMode))))

(event Custom|checkForMovement
  (bind _returnvalue (Game|GetPlayerController 0))
  (bind (_deltax _deltay) (Class|PlayerController|GetInputMouseDelta _returnvalue))
  ;[1 1 1] Mode to rotate and edit cube -Rob
  (if (and (Variables|Default|GetmouseIsPressed) (Variables|Default|GetclickOffCube))
    (Transformation|AddWorldRotation (Variables|Default|GetDefaultSceneRoot) (Math|Rotator|MakeRotator 0.0 (* _deltay -1e+01) (* _deltax -1e+01)) false false)))

(event Custom|toggleButtonVisibility
  ;[1 1 1] Toggles visibility of buttons -Rob
  (Rendering|SetVisibility (Variables|Default|GetButtonA) (not (Variables|Default|GetbuttonsVisible)) false)
  (Variables|Default|SetbuttonsVisible (not (Variables|Default|GetbuttonsVisible))))

(event MouseInput|EventActorOnClicked
  (params (ButtonPressed :type Key%20Structure :default "None"))
  ;[1 1 1] Checks whether the mouse is clicked on/off the cube -Rob
  (Variables|Default|SetclickOffCube false))

(event EventBeginPlay
  (bind _cubeg (Variables|Default|GetCubeG))
  (bind _cubeh (Variables|Default|GetCubeH))
  (bind _cubea (Variables|Default|GetCubeA))
  (bind _cubee (Variables|Default|GetCubeE))
  (bind _cubef (Variables|Default|GetCubeF))
  (bind _cubeg_2 (Variables|Default|GetCubeG))
  (bind _cubeh_2 (Variables|Default|GetCubeH))
  (bind _cubeb (Variables|Default|GetCubeB))
  (bind _cubeb_2 (Variables|Default|GetCubeB))
  (bind _cubea_2 (Variables|Default|GetCubeA))
  (bind _cubee_2 (Variables|Default|GetCubeE))
  (bind _cubef_2 (Variables|Default|GetCubeF))
  (bind _cubea_3 (Variables|Default|GetCubeA))
  (bind _cubeh_3 (Variables|Default|GetCubeH))
  (bind _cubec (Variables|Default|GetCubeC))
  (bind _cubec_2 (Variables|Default|GetCubeC))
  (bind _cubec_3 (Variables|Default|GetCubeC))
  (bind _cubed (Variables|Default|GetCubeD))
  (bind _cubeb_3 (Variables|Default|GetCubeB))
  (bind _cubed_2 (Variables|Default|GetCubeD))
  (bind _cubed_3 (Variables|Default|GetCubeD))
  (bind _cubeg_3 (Variables|Default|GetCubeG))
  (bind _cubee_3 (Variables|Default|GetCubeE))
  (bind _cubef_3 (Variables|Default|GetCubeF))
  (bind _array (Utilities|Array|MakeArray _cubea _cubeb _cubec_3 _cubed_2))
  (bind _array_2 (Utilities|Array|MakeArray _cubeb_3 _cubee_3 _cubed_3 _cubeg_3))
  (bind _array_3 (Utilities|Array|MakeArray _cubee _cubef _cubeg_2 _cubeh_2))
  (bind _array_4 (Utilities|Array|MakeArray _cubea_2 _cubef_3 _cubeb_2 _cubee_2))
  (bind _array_5 (Utilities|Array|MakeArray _cubec _cubeh_3 _cubea_3 _cubef_2))
  (bind _array_6 (Utilities|Array|MakeArray _cubed _cubeg _cubec_2 _cubeh))
  ;[1 1 1] Face array initialization - Rob
  (Utilities|FlowControl|Sequence
    (:then_0
      (Utilities|Array|AppendArray (Variables|Default|GetfaceA) _array_2)
      (Utilities|Array|AppendArray (Variables|Default|GetfaceAanswer) _array_2))
    (:then_1
      (Utilities|Array|AppendArray (Variables|Default|GetfaceB) _array)
      (Utilities|Array|AppendArray (Variables|Default|GetfaceBanswer) _array))
    (:then_2
      (Utilities|Array|AppendArray (Variables|Default|GetfaceC) _array_3)
      (Utilities|Array|AppendArray (Variables|Default|GetfaceCanswer) _array_3))
    (:then_3
      (Utilities|Array|AppendArray (Variables|Default|GetfaceD) _array_4)
      (Utilities|Array|AppendArray (Variables|Default|GetfaceDanswer) _array_4))
    (:then_4
      (Utilities|Array|AppendArray (Variables|Default|GetfaceE) _array_5)
      (Utilities|Array|AppendArray (Variables|Default|GetfaceEanswer) _array_5))
    (:then_5
      (Utilities|Array|AppendArray (Variables|Default|GetfaceF) _array_6)
      (Utilities|Array|AppendArray (Variables|Default|GetfaceFanswer) _array_6))
    (:then_6
      ;[1 1 1] Set Initial Rotations
      (for _array_element (Variables|Default|GetInitialRots)
        (CallFunction|FaceRot _array_element)))))

(event Input|ActionEvents|InputActionEquip
  (params (Key :type Key%20Structure :default "None"))
  ;[1 1 1] Everything I changed is in this box -Ben
  (:Pressed
    (Utilities|FlowControl|Gate true
      (:Exit
        ;;[1 1 1] isSolved is set to true on default
        (if (Variables|Default|GetisSolved)
          (Variables|Default|SetisEquipped true)
          (Default|EquipItem (Variables|Default|GetCharacter) 1))))))

(event Input|MouseEvents|LeftMouseButton
  (params (Key :type Key%20Structure :default "None"))
  ;[1 1 1] Checks whether the mouse is clicked on/off the cube -Rob
  (:Pressed
    (Variables|Default|SetmouseIsPressed true))
  (:Released
    (Variables|Default|SetmouseIsPressed false)
    (Variables|Default|SetclickOffCube true)))

(fn ConstructionScript)

(fn CubeSolveMode
  ;[1 1 1] Toggle function for Rubiks cube "puzzle solving mode"
  (if (Variables|Default|GetisInCubeSolveMode)
    (CallFunction|SetSolveModeOff)
    (else
      (CallFunction|SetSolveModeon))))

(fn FaceRot
  (params (faceLetter :type String))
  (bind _facec (Variables|Default|GetfaceC))
  (bind _faced (Variables|Default|GetfaceD))
  (bind _facef (Variables|Default|GetfaceF))
  (bind _faceb (Variables|Default|GetfaceB))
  (bind _facee (Variables|Default|GetfaceE))
  (bind _facee_2 (Variables|Default|GetfaceE))
  (bind _facef_2 (Variables|Default|GetfaceF))
  (bind _faced_2 (Variables|Default|GetfaceD))
  (bind _facea (Variables|Default|GetfaceA))
  (bind _facec_2 (Variables|Default|GetfaceC))
  (bind _faceb_2 (Variables|Default|GetfaceB))
  (bind _faced_3 (Variables|Default|GetfaceD))
  (bind _facea_2 (Variables|Default|GetfaceA))
  (bind _facec_3 (Variables|Default|GetfaceC))
  (bind _facef_3 (Variables|Default|GetfaceF))
  (bind _facec_4 (Variables|Default|GetfaceC))
  (bind _facef_4 (Variables|Default|GetfaceF))
  (bind _facea_3 (Variables|Default|GetfaceA))
  (bind _facee_3 (Variables|Default|GetfaceE))
  (bind _faceb_3 (Variables|Default|GetfaceB))
  (bind _faced_4 (Variables|Default|GetfaceD))
  (bind _facea_4 (Variables|Default|GetfaceA))
  (bind _facee_4 (Variables|Default|GetfaceE))
  (bind _faceb_4 (Variables|Default|GetfaceB))
  (bind _faced_5 (Variables|Default|GetfaceD))
  (bind _facec_5 (Variables|Default|GetfaceC))
  (bind _facee_5 (Variables|Default|GetfaceE))
  (bind _facea_5 (Variables|Default|GetfaceA))
  (bind _faceb_5 (Variables|Default|GetfaceB))
  (bind _facef_5 (Variables|Default|GetfaceF))
  ;[1 1 1] Rotatates faces/cubes, face A's comments apply to each face section -Rob
  (switch string faceLetter
    (:A
      ;;[1 1 1] Rotates all cubes under the Face A array
      (for _array_element (Variables|Default|GetfaceA)
        (Transformation|SetRelativeRotation _array_element (Math|Rotator|MakeRotationfromAxes (Math|Vector|Normalize (.X (Math|Rotator|BreakRotIntoAxes (Math|Rotator|CombineRotators (Variables|/Script/Engine.SceneComponent|GetRelativeRotation _array_element) "0.000000, 0,90.000000")))) (Math|Vector|Normalize (.Y (Math|Rotator|BreakRotIntoAxes (Math|Rotator|CombineRotators (Variables|/Script/Engine.SceneComponent|GetRelativeRotation _array_element) "0.000000, 0,90.000000")))) (Math|Vector|Normalize (.Z (Math|Rotator|BreakRotIntoAxes (Math|Rotator|CombineRotators (Variables|/Script/Engine.SceneComponent|GetRelativeRotation _array_element) "0.000000, 0,90.000000"))))) false false))
      (Utilities|FlowControl|Sequence
        (:then_0
          ;;[1 1 1] Saves the current face before any editing - used in finding other face array's updated values
          (Utilities|Array|AppendArray (Variables|Default|GettempFace) (Variables|Default|GetfaceA)))
        (:then_1
          ;;[1 1 1] Updates order of cubes in currently rotated face
          (Utilities|Array|Swap _facea_2 0 2)
          (Utilities|Array|Insert _facea_2 (Utilities|Array|Get(acopy) _facea_2 1) 4)
          (Utilities|Array|RemoveIndex _facea_2 1))
        (:then_2
          ;;[1 1 1] Goes over each adjacent face's array, updating what cubes they now have
          (Utilities|Array|Swap _facec_3 0 2)
          (Utilities|Array|SetArrayElem _facec_3 0 (Utilities|Array|Get(acopy) (Variables|Default|GettempFace))))
        (:then_3
          (Utilities|Array|Swap _facef_3 1)
          (Utilities|Array|SetArrayElem _facef_3 1 (Utilities|Array|Get(acopy) (Variables|Default|GettempFace) 1)))
        (:then_4
          (Utilities|Array|Swap _faced_3 2 3)
          (Utilities|Array|SetArrayElem _faced_3 2 (Utilities|Array|Get(acopy) (Variables|Default|GettempFace) 2)))
        (:then_5
          (Utilities|Array|Swap _faceb_2 3 1)
          (Utilities|Array|SetArrayElem _faceb_2 3 (Utilities|Array|Get(acopy) (Variables|Default|GettempFace) 3)))
        (:then_6
          ;;[1 1 1] Clear the temp face for the next rotation
          (Utilities|Array|Clear (Variables|Default|GettempFace)))))
    (:B
      (for _array_element_2 (Variables|Default|GetfaceB)
        (Transformation|SetRelativeRotation _array_element_2 (Math|Rotator|MakeRotationfromAxes (Math|Vector|Normalize (.X (Math|Rotator|BreakRotIntoAxes (Math|Rotator|CombineRotators (Variables|/Script/Engine.SceneComponent|GetRelativeRotation _array_element_2) "90.000000, 0,0.000000")))) (Math|Vector|Normalize (.Y (Math|Rotator|BreakRotIntoAxes (Math|Rotator|CombineRotators (Variables|/Script/Engine.SceneComponent|GetRelativeRotation _array_element_2) "90.000000, 0,0.000000")))) (Math|Vector|Normalize (.Z (Math|Rotator|BreakRotIntoAxes (Math|Rotator|CombineRotators (Variables|/Script/Engine.SceneComponent|GetRelativeRotation _array_element_2) "90.000000, 0,0.000000"))))) false false))
      (Utilities|FlowControl|Sequence
        (:then_0
          (Utilities|Array|AppendArray (Variables|Default|GettempFace) (Variables|Default|GetfaceB)))
        (:then_1
          (Utilities|Array|Swap _faceb_3 0 2)
          (Utilities|Array|Insert _faceb_3 (Utilities|Array|Get(acopy) _faceb_3 1) 4)
          (Utilities|Array|RemoveIndex _faceb_3 1))
        (:then_2
          (Utilities|Array|Swap _facea_4 0 2)
          (Utilities|Array|SetArrayElem _facea_4 0 (Utilities|Array|Get(acopy) (Variables|Default|GettempFace))))
        (:then_3
          (Utilities|Array|Swap _facef_4 0 2)
          (Utilities|Array|SetArrayElem _facef_4 0 (Utilities|Array|Get(acopy) (Variables|Default|GettempFace) 1)))
        (:then_4
          (Utilities|Array|Swap _faced_4 0 2)
          (Utilities|Array|SetArrayElem _faced_4 0 (Utilities|Array|Get(acopy) (Variables|Default|GettempFace) 2)))
        (:then_5
          (Utilities|Array|Swap _facee_4 0 2)
          (Utilities|Array|SetArrayElem _facee_4 0 (Utilities|Array|Get(acopy) (Variables|Default|GettempFace) 3)))
        (:then_6
          (Utilities|Array|Clear (Variables|Default|GettempFace)))))
    (:C
      (for _array_element_3 (Variables|Default|GetfaceC)
        (Transformation|SetRelativeRotation _array_element_3 (Math|Rotator|MakeRotationfromAxes (Math|Vector|Normalize (.X (Math|Rotator|BreakRotIntoAxes (Math|Rotator|CombineRotators (Variables|/Script/Engine.SceneComponent|GetRelativeRotation _array_element_3) "-90.000000, 0,0.000000")))) (Math|Vector|Normalize (.Y (Math|Rotator|BreakRotIntoAxes (Math|Rotator|CombineRotators (Variables|/Script/Engine.SceneComponent|GetRelativeRotation _array_element_3) "-90.000000, 0,0.000000")))) (Math|Vector|Normalize (.Z (Math|Rotator|BreakRotIntoAxes (Math|Rotator|CombineRotators (Variables|/Script/Engine.SceneComponent|GetRelativeRotation _array_element_3) "-90.000000, 0,0.000000"))))) false false))
      (Utilities|FlowControl|Sequence
        (:then_0
          (Utilities|Array|AppendArray (Variables|Default|GettempFace) (Variables|Default|GetfaceC)))
        (:then_1
          (Utilities|Array|Swap _facec_2 0 2)
          (Utilities|Array|Insert _facec_2 (Utilities|Array|Get(acopy) _facec_2 1) 4)
          (Utilities|Array|RemoveIndex _facec_2 1))
        (:then_2
          (Utilities|Array|Swap _facee_2 1 3)
          (Utilities|Array|SetArrayElem _facee_2 3 (Utilities|Array|Get(acopy) (Variables|Default|GettempFace))))
        (:then_3
          (Utilities|Array|Swap _facef_2 1 3)
          (Utilities|Array|SetArrayElem _facef_2 3 (Utilities|Array|Get(acopy) (Variables|Default|GettempFace) 1)))
        (:then_4
          (Utilities|Array|Swap _faced_2 1 3)
          (Utilities|Array|SetArrayElem _faced_2 3 (Utilities|Array|Get(acopy) (Variables|Default|GettempFace) 2)))
        (:then_5
          (Utilities|Array|Swap _facea 3 1)
          (Utilities|Array|SetArrayElem _facea 3 (Utilities|Array|Get(acopy) (Variables|Default|GettempFace) 3)))
        (:then_6
          (Utilities|Array|Clear (Variables|Default|GettempFace)))))
    (:D
      (for _array_element_4 (Variables|Default|GetfaceD)
        (Transformation|SetRelativeRotation _array_element_4 (Math|Rotator|MakeRotationfromAxes (Math|Vector|Normalize (.X (Math|Rotator|BreakRotIntoAxes (Math|Rotator|CombineRotators (Variables|/Script/Engine.SceneComponent|GetRelativeRotation _array_element_4) "0.000000,90.000000,0.000000")))) (Math|Vector|Normalize (.Y (Math|Rotator|BreakRotIntoAxes (Math|Rotator|CombineRotators (Variables|/Script/Engine.SceneComponent|GetRelativeRotation _array_element_4) "0.000000,90.000000,0.000000")))) (Math|Vector|Normalize (.Z (Math|Rotator|BreakRotIntoAxes (Math|Rotator|CombineRotators (Variables|/Script/Engine.SceneComponent|GetRelativeRotation _array_element_4) "0.000000,90.000000,0.000000"))))) false false))
      (Utilities|FlowControl|Sequence
        (:then_0
          (Utilities|Array|AppendArray (Variables|Default|GettempFace) (Variables|Default|GetfaceD)))
        (:then_1
          (Utilities|Array|Swap _faced_5 0 2)
          (Utilities|Array|Insert _faced_5 (Utilities|Array|Get(acopy) _faced_5 1) 4)
          (Utilities|Array|RemoveIndex _faced_5 1))
        (:then_2
          (Utilities|Array|Swap _facec_4 0 1)
          (Utilities|Array|SetArrayElem _facec_4 1 (Utilities|Array|Get(acopy) (Variables|Default|GettempFace))))
        (:then_3
          (Utilities|Array|Swap _facea_3 1)
          (Utilities|Array|SetArrayElem _facea_3 1 (Utilities|Array|Get(acopy) (Variables|Default|GettempFace) 1)))
        (:then_4
          (Utilities|Array|Swap _facee_3 2 3)
          (Utilities|Array|SetArrayElem _facee_3 2 (Utilities|Array|Get(acopy) (Variables|Default|GettempFace) 2)))
        (:then_5
          (Utilities|Array|Swap _faceb_4 0 1)
          (Utilities|Array|SetArrayElem _faceb_4 1 (Utilities|Array|Get(acopy) (Variables|Default|GettempFace) 3)))
        (:then_6
          (Utilities|Array|Clear (Variables|Default|GettempFace)))))
    (:E
      (for _array_element_5 (Variables|Default|GetfaceE)
        (Transformation|SetRelativeRotation _array_element_5 (Math|Rotator|MakeRotationfromAxes (Math|Vector|Normalize (.X (Math|Rotator|BreakRotIntoAxes (Math|Rotator|CombineRotators (Variables|/Script/Engine.SceneComponent|GetRelativeRotation _array_element_5) "0.000000, 0,-90.000000")))) (Math|Vector|Normalize (.Y (Math|Rotator|BreakRotIntoAxes (Math|Rotator|CombineRotators (Variables|/Script/Engine.SceneComponent|GetRelativeRotation _array_element_5) "0.000000, 0,-90.000000")))) (Math|Vector|Normalize (.Z (Math|Rotator|BreakRotIntoAxes (Math|Rotator|CombineRotators (Variables|/Script/Engine.SceneComponent|GetRelativeRotation _array_element_5) "0.000000, 0,-90.000000"))))) false false))
      (Utilities|FlowControl|Sequence
        (:then_0
          (Utilities|Array|AppendArray (Variables|Default|GettempFace) (Variables|Default|GetfaceE)))
        (:then_1
          (Utilities|Array|Swap _facee 0 2)
          (Utilities|Array|Insert _facee (Utilities|Array|Get(acopy) _facee 1) 4)
          (Utilities|Array|RemoveIndex _facee 1))
        (:then_2
          (Utilities|Array|Swap _facec 1 3)
          (Utilities|Array|SetArrayElem _facec 3 (Utilities|Array|Get(acopy) (Variables|Default|GettempFace))))
        (:then_3
          (Utilities|Array|Swap _faced 1)
          (Utilities|Array|SetArrayElem _faced 1 (Utilities|Array|Get(acopy) (Variables|Default|GettempFace) 1)))
        (:then_4
          (Utilities|Array|Swap _facef 2 3)
          (Utilities|Array|SetArrayElem _facef 2 (Utilities|Array|Get(acopy) (Variables|Default|GettempFace) 2)))
        (:then_5
          (Utilities|Array|Swap _faceb 0 2)
          (Utilities|Array|SetArrayElem _faceb 0 (Utilities|Array|Get(acopy) (Variables|Default|GettempFace) 3)))
        (:then_6
          (Utilities|Array|Clear (Variables|Default|GettempFace)))))
    (:F
      (for _array_element_6 (Variables|Default|GetfaceF)
        (Transformation|SetRelativeRotation _array_element_6 (Math|Rotator|MakeRotationfromAxes (Math|Vector|Normalize (.X (Math|Rotator|BreakRotIntoAxes (Math|Rotator|CombineRotators (Variables|/Script/Engine.SceneComponent|GetRelativeRotation _array_element_6) "0.000000,-90.000000,0.000000")))) (Math|Vector|Normalize (.Y (Math|Rotator|BreakRotIntoAxes (Math|Rotator|CombineRotators (Variables|/Script/Engine.SceneComponent|GetRelativeRotation _array_element_6) "0.000000,-90.000000,0.000000")))) (Math|Vector|Normalize (.Z (Math|Rotator|BreakRotIntoAxes (Math|Rotator|CombineRotators (Variables|/Script/Engine.SceneComponent|GetRelativeRotation _array_element_6) "0.000000,-90.000000,0.000000"))))) false false))
      (Utilities|FlowControl|Sequence
        (:then_0
          (Utilities|Array|AppendArray (Variables|Default|GettempFace) (Variables|Default|GetfaceF)))
        (:then_1
          (Utilities|Array|Swap _facef_5 0 2)
          (Utilities|Array|Insert _facef_5 (Utilities|Array|Get(acopy) _facef_5 1) 4)
          (Utilities|Array|RemoveIndex _facef_5 1))
        (:then_2
          (Utilities|Array|Swap _facec_5 2 3)
          (Utilities|Array|SetArrayElem _facec_5 2 (Utilities|Array|Get(acopy) (Variables|Default|GettempFace))))
        (:then_3
          (Utilities|Array|Swap _facee_5 1)
          (Utilities|Array|SetArrayElem _facee_5 1 (Utilities|Array|Get(acopy) (Variables|Default|GettempFace) 1)))
        (:then_4
          (Utilities|Array|Swap _facea_5 2 3)
          (Utilities|Array|SetArrayElem _facea_5 2 (Utilities|Array|Get(acopy) (Variables|Default|GettempFace) 2)))
        (:then_5
          (Utilities|Array|Swap _faceb_5 2 3)
          (Utilities|Array|SetArrayElem _faceb_5 2 (Utilities|Array|Get(acopy) (Variables|Default|GettempFace) 3)))
        (:then_6
          (Utilities|Array|Clear (Variables|Default|GettempFace)))))))

(fn IsWin
  ;[1 1 1] Loop through and check if each face is correct for the win condition -Rob
  (bind _isequal (CallFunction|ArrayIsEqual (Variables|Default|GetfaceA) (Variables|Default|GetfaceAanswer)))
  (if _isequal
    (bind _isequal_2 (CallFunction|ArrayIsEqual (Variables|Default|GetfaceB) (Variables|Default|GetfaceBanswer)))
    (if _isequal_2
      (bind _isequal_3 (CallFunction|ArrayIsEqual (Variables|Default|GetfaceC) (Variables|Default|GetfaceCanswer)))
      (if _isequal_3
        (bind _isequal_4 (CallFunction|ArrayIsEqual (Variables|Default|GetfaceD) (Variables|Default|GetfaceDanswer)))
        (if _isequal_4
          (bind _isequal_5 (CallFunction|ArrayIsEqual (Variables|Default|GetfaceE) (Variables|Default|GetfaceEanswer)))
          (if _isequal_5
            (bind _isequal_6 (CallFunction|ArrayIsEqual (Variables|Default|GetfaceF) (Variables|Default|GetfaceFanswer)))
            (if _isequal_6
              (Variables|Default|SetisSolved true)
              (CallFunction|SetSolveModeOff)
              (Audio|PlaySoundatLocation "/Game/Rob/UsedSounds/VR_click1.VR_click1" (Transformation|GetActorLocation) "0, 0, 0" 1.0 1.0 0.0 0 0 0)
              (Rendering|SetVisibility (Variables|Default|GetPointLight) true false)
              (return)
              (else
                (return)))
            (else
              (return)))
          (else
            (return)))
        (else
          (return)))
      (else
        (return)))
    (else
      (return))))

(fn ArrayIsEqual
  (params (ArrayA :type Array%20of%20Static%20Mesh%20Component%20Object%20References) (ArrayB :type Array%20of%20Static%20Mesh%20Component%20Object%20References))
  (for (_array_element _array_index) ArrayA
    (if (not (Utilities|Enum|Equal(Enum) (Utilities|GetObjectName _array_element) (Utilities|GetObjectName (Utilities|Array|Get(acopy) ArrayB _array_index))))
      (return false)))
  (return true))