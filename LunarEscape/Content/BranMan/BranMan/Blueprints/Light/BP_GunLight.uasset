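; BP_GunLight is a light actor that switches from red to green when shot.
; It flags itself red on BeginPlay and calls ChangeLight when a BP_Bullet overlaps it.
; ChangeLight recolors the spot light, swaps a mesh material slot to GreenGlow, clears the flag and prints a debug message.
; The change is one-way, as nothing after BeginPlay sets the flag back to red.
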(event EventBeginPlay
  (Variables|Default|SetIsLightRed true))

(event Collision|EventActorBeginOverlap
  (params (OtherActor :type Actor%20Object%20Reference))
  (Utilities|Casting|CastToBP_Bullet OtherActor)
  (CallFunction|ChangeLight))

(event EventTick
  (params (DeltaSeconds :type Float%20%28single-precision%29)))

(fn ConstructionScript)

(fn ChangeLight
  (if (Variables|Default|GetIsLightRed)
    (Rendering|Components|Light|SetLightColor (Variables|Default|GetSpotLight) "(R=0.000000,G=255.000000,B=0.000000,A=1.000000)" true)
    (Rendering|Material|SetMaterial (Variables|Default|GetStaticMesh) 1 "/Game/BranMan/BranMan/Blueprints/Light/GreenGlow.GreenGlow")
    (Variables|Default|SetIsLightRed false)
    (Development|PrintString "Light is now green")))