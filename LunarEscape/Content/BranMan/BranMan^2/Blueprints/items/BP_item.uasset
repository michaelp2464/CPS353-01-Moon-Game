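; BP_item is an interactable item that shows an on-screen text prompt when a player comes within interaction range.
; On range entry, it creates an interaction widget for that player inside a screen-space widget component added at runtime, then destroys the component on exit.
; GetInteractionText and GetInteractionTextAttach supply the default "Interact" label and root attach point.
; OnInteracted is an empty stub.
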(event EventOnINtewractionRangeExited
  ;[1 1 1] Destroys text box when range is exited
  (bind _interactionwidgetcomponent (Variables|Default|GetInteractionWidgetComponent)
    (:then
      (Components|DestroyComponent _interactionwidgetcomponent))
    (:else)))

(event EventOnInteractionRangeEntered
  (params (Player :type Third%20Person%20Character%20Object%20Reference))
  ;[1 1 1] Attach widget (Text box that say interact) to item when player is near
  (Variables|Default|GetInteractionWidgetComponent
    (:then)
    (:else
      (bind _asplayer_controller (Utilities|Casting|CastToPlayerController (Pawn|GetController Player)))
      (bind _returnvalue (UserInterface|CreateWidget "/Game/BranMan/BranMan^2/Blueprints/items/InteractionWidget.InteractionWidget_C" _asplayer_controller (Private|GetInteractionText)))
      (bind _returnvalue_2 (AddComponent|AddWidgetComponent false))
      (bind _output_get (Variables|Default|SetInteractionWidgetComponent _returnvalue_2))
      (UserInterface|SetWidget _output_get _returnvalue)
      (Class|WidgetComponent|SetWidgetSpace _output_get "Screen")
      (Class|WidgetComponent|SetDrawatDesiredSize _output_get true)
      (Collision|SetCollisionEnabled _output_get "NoCollision")
      (Transformation|AttachComponentToComponent _output_get (Private|GetInteractionTextAttach) "None" "SnapToTarget" "SnapToTarget" "SnapToTarget" true))))

(event EventOnInteracted
  (params (Player :type Third%20Person%20Character%20Object%20Reference)))

(fn ConstructionScript)

(fn GetInteractionTextAttach
  (return (Variables|Default|GetDefaultSceneRoot)))

(fn GetInteractionText
  (return "Interact"))