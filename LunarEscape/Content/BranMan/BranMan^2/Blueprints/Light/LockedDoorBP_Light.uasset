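; Locked door Blueprint that swings open when the player interacts while holding an equipped key and its two lights are not both red.
; Overlap handlers enable or disable input and toggle a gate for the player character.
; A failed light or key check plays a locked sound; success plays an opening sound and flip-flops a timeline that lerps door yaw.
; Timeline updates also disable the door's input.
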(event Custom|CustomEvent
  (params (OverlappedComponent :type Primitive%20Component%20Object%20Reference) (OtherActor :type Actor%20Object%20Reference) (OtherComp :type Primitive%20Component%20Object%20Reference) (OtherBodyIndex :type Integer))
  ;[1 1 1] If the player shot all of the moving lights
  (Utilities|Casting|CastToThirdPersonCharacter OtherActor)
  (Input|DisableInput (Game|GetPlayerController 0))
  (Utilities|FlowControl|Gate true) ; enters at Close
)

(event Custom|CustomEvent_1
  (params (OverlappedComponent :type Primitive%20Component%20Object%20Reference) (OtherActor :type Actor%20Object%20Reference) (OtherComp :type Primitive%20Component%20Object%20Reference) (OtherBodyIndex :type Integer) (bFromSweep :type Boolean) (SweepResult :type Hit%20Result%20Structure%20%28by%20ref%29))
  ;[1 1 1] If the player shot all of the moving lights
  (bind _asthird_person_character (Utilities|Casting|CastToThirdPersonCharacter OtherActor))
  (Input|EnableInput (Game|GetPlayerController 0))
  (Utilities|FlowControl|Gate true) ; enters at Open
)

(event Input|ActionEvents|InputActionInteract
  (params (Key :type Key%20Structure :default "None"))
  ;[1 1 1] If the player shot all of the moving lights
  (:Pressed
    (bind _askey_bp (Utilities|Casting|CastToKeyBP (Variables|/Game/ThirdPersonBP/Blueprints/ThirdPersonCharacter.ThirdPersonCharacter_C|GetKey (stale Custom|CustomEvent_1 _asthird_person_character))))
    (if (and (Math|Boolean|NANDBoolean (Variables|/Game/BranMan/BranMan^2/Blueprints/Light/BP_GunLight.BP_GunLight_C|GetIsLightRed (Variables|Default|GetLight1)) (Variables|/Game/BranMan/BranMan^2/Blueprints/Light/BP_GunLight.BP_GunLight_C|GetIsLightRed (Variables|Default|GetLight2))) (Variables|/Game/Ben/B_Blueprints/KeyBP.KeyBP_C|GetisEquipped _askey_bp))
      (Utilities|FlowControl|Gate true
        (:Exit
          (Audio|PlaySoundatLocation "/Game/Ben/B_Sounds/door_open.door_open" (Transformation|GetActorLocation) "0, 0, 0" 1.0 1.0 0.65 0 0 0)
          ;[1 1 1] ...run the door opening animation
          (Utilities|FlowControl|FlipFlop
            (:A
              ;;[1 1 1] Open/Open animation backwards
              (bind _door_open_close (Timeline|Timeline_0 Play)
                (:Update
                  (Transformation|SetRelativeRotation (Variables|Default|GetDoor) (Math|Rotator|MakeRotator 0.0 0.0 (Math|Float|Lerp (Variables|Default|GetClosed) (Variables|Default|GetOpen) _door_open_close)) false false)
                  (Input|DisableInput (Game|GetPlayerController 0)))))
            (:B
              (Timeline|Timeline_0 Reverse)))))
      (else
        (Audio|PlaySoundatLocation "/Game/Ben/B_Sounds/door_locked.door_locked" (Transformation|GetActorLocation) "0, 0, 0" 1.0 1.0 0.0 0 0 0)))))

(fn ConstructionScript)