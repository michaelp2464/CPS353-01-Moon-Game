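; Sliding glass door pair that opens with sound for the ThirdPersonCharacter and can also be opened by an Activate_Door event.
; On overlap, Timeline_0 slides both panels apart, then reverses after a short delay on exit.
; Overlap movement is skipped only when all three linked lights are red and Keypad.DoorOpened is true.
; Activate_Door uses a separate timeline with no reverse, so it only opens.
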(event Custom|Activate_Door
  (Audio|PlaySoundatLocation "/Game/Joshua/Sounds/Slidingdoor_Sounds/Sci-Fi_Sliding_Door_Cue.Sci-Fi_Sliding_Door_Cue" (Transformation|GetWorldLocation (Variables|Default|GetGlassDoorA)) "0, 0, 0" 1.0 1.0 0.0 0 0 0)
  (bind _newtrack_0 (Timeline|Timeline_1 Play)
    (:Update
      (Transformation|SetRelativeLocation (Variables|Default|GetGlassDoorB) (Math|Vector|Lerp(Vector) "0, 0, 0" "170.000000, 0, 0" _newtrack_0) false false)
      (Transformation|SetRelativeLocation (Variables|Default|GetGlassDoorA) (Math|Vector|Lerp(Vector) "-361.000000,69.999992, 0" "-535.000000,69.999878, 0" _newtrack_0) false false))))

(event Collision|EventActorBeginOverlap
  (params (OtherActor :type Actor%20Object%20Reference))
  (Utilities|Casting|CastToThirdPersonCharacter OtherActor)
  (bind _alllightsgreen_ (CallFunction|LightStatus))
  (if (or _alllightsgreen_ (not (Variables|/Game/Mikey/Blueprints/BP_Keypad.BP_Keypad_C|Getdoor_opened (Variables|Default|GetKeypad))))
    (Audio|PlaySoundatLocation "/Game/Joshua/Sounds/Slidingdoor_Sounds/Sci-Fi_Sliding_Door_Cue.Sci-Fi_Sliding_Door_Cue" (Transformation|GetWorldLocation (Variables|Default|GetGlassDoorA)) "0, 0, 0" 1.0 1.0 0.0 0 0 0)
    (bind _newtrack_0 (Timeline|Timeline_0 Play)
      (:Update
        (Transformation|SetRelativeLocation (Variables|Default|GetGlassDoorB) (Math|Vector|Lerp(Vector) "0, 0, 0" "170.000000, 0, 0" _newtrack_0) false false)
        (Transformation|SetRelativeLocation (Variables|Default|GetGlassDoorA) (Math|Vector|Lerp(Vector) "-361.000000,69.999992, 0" "-535.000000,69.999878, 0" _newtrack_0) false false)))))

(event Collision|EventActorEndOverlap
  (params (OtherActor :type Actor%20Object%20Reference))
  (Utilities|Casting|CastToThirdPersonCharacter OtherActor)
  (bind _alllightsgreen_ (CallFunction|LightStatus))
  (if (or _alllightsgreen_ (not (Variables|/Game/Mikey/Blueprints/BP_Keypad.BP_Keypad_C|Getdoor_opened (Variables|Default|GetKeypad))))
    (Utilities|FlowControl|Delay 1.0)
    (Utilities|FlowControl|Sequence
      (:then_0
        (bind _newtrack_0 (Timeline|Timeline_0 Reverse)
          (:Update
            (Transformation|SetRelativeLocation (Variables|Default|GetGlassDoorB) (Math|Vector|Lerp(Vector) "0, 0, 0" "170.000000, 0, 0" _newtrack_0) false false)
            (Transformation|SetRelativeLocation (Variables|Default|GetGlassDoorA) (Math|Vector|Lerp(Vector) "-361.000000,69.999992, 0" "-535.000000,69.999878, 0" _newtrack_0) false false))))
      (:then_1
        (Utilities|FlowControl|Delay 0.7)
        (Audio|PlaySoundatLocation "/Game/Joshua/Sounds/Slidingdoor_Sounds/Sci-Fi_Sliding_Door_Cue.Sci-Fi_Sliding_Door_Cue" (Transformation|GetWorldLocation (Variables|Default|GetGlassDoorA)) "0, 0, 0" 1.0 1.0 0.0 0 0 0)))))

(fn ConstructionScript)

(fn LightStatus
  (if (Math|Boolean|ANDBoolean (Variables|/Game/BranMan/BranMan^2/Blueprints/Light/BP_GunLight.BP_GunLight_C|GetIsLightRed (Variables|Default|GetLight1)) (Variables|/Game/BranMan/BranMan^2/Blueprints/Light/BP_GunLight.BP_GunLight_C|GetIsLightRed (Variables|Default|GetLight2)) (Variables|/Game/BranMan/BranMan^2/Blueprints/Light/BP_GunLight.BP_GunLight_C|GetIsLightRed (Variables|Default|GetLight3)))
    (return false)
    (else
      (return true))))