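; Sliding double glass door meant to open for the third-person character based on an ordered state of three lights.
; Overlap begin and end call LightStatus to gate a timeline that slides both panels with sound, reversing after a delay.
; LightStatus nests contradictory red-state checks, so as written it always resets all lights red and never passes.
; Activate_Door opens the panels through a separate timeline, bypassing the light check.
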(event Custom|Activate_Door
  (Audio|PlaySoundatLocation "/Game/Joshua/Sounds/Slidingdoor_Sounds/Sci-Fi_Sliding_Door_Cue.Sci-Fi_Sliding_Door_Cue" (Transformation|GetWorldLocation (Variables|Default|GetGlassDoorA)) "0, 0, 0" 1.0 1.0 0.0 0 0 0)
  (bind _newtrack_0 (Timeline|Timeline_1 Play)
    (:Update
      (Transformation|SetRelativeLocation (Variables|Default|GetGlassDoorB) (Math|Vector|Lerp(Vector) "0, 0, 0" "170.000000, 0, 0" _newtrack_0) false false)
      (Transformation|SetRelativeLocation (Variables|Default|GetGlassDoorA) (Math|Vector|Lerp(Vector) "-361.000000,69.999992, 0" "-535.000000,69.999878, 0" _newtrack_0) false false))))

(event Collision|EventActorBeginOverlap
  (params (OtherActor :type Actor%20Object%20Reference))
  (Utilities|Casting|CastToThirdPersonCharacter OtherActor)
  (bind _alllightsgreen_ (CallFunction|LightStatus))
  (if _alllightsgreen_
    (Development|PrintString "All Lights Are Green!")
    (Audio|PlaySoundatLocation "/Game/Joshua/Sounds/Slidingdoor_Sounds/Sci-Fi_Sliding_Door_Cue.Sci-Fi_Sliding_Door_Cue" (Transformation|GetWorldLocation (Variables|Default|GetGlassDoorA)) "0, 0, 0" 1.0 1.0 0.0 0 0 0)
    (bind _newtrack_0 (Timeline|Timeline_0 Play)
      (:Update
        (Transformation|SetRelativeLocation (Variables|Default|GetGlassDoorB) (Math|Vector|Lerp(Vector) "0, 0, 0" "170.000000, 0, 0" _newtrack_0) false false)
        (Transformation|SetRelativeLocation (Variables|Default|GetGlassDoorA) (Math|Vector|Lerp(Vector) "-361.000000,69.999992, 0" "-535.000000,69.999878, 0" _newtrack_0) false false)))))

(event Collision|EventActorEndOverlap
  (params (OtherActor :type Actor%20Object%20Reference))
  (Utilities|Casting|CastToThirdPersonCharacter OtherActor)
  (bind _alllightsgreen_ (CallFunction|LightStatus))
  (if _alllightsgreen_
    (Utilities|FlowControl|Delay 1.0)
    (Utilities|FlowControl|Sequence
      (:then_0
        (bind _newtrack_0 (Timeline|Timeline_0 Reverse)
          (:Update
            (Transformation|SetRelativeLocation (Variables|Default|GetGlassDoorB) (Math|Vector|Lerp(Vector) "0, 0, 0" "170.000000, 0, 0" _newtrack_0) false false)
            (Transformation|SetRelativeLocation (Variables|Default|GetGlassDoorA) (Math|Vector|Lerp(Vector) "-361.000000,69.999992, 0" "-535.000000,69.999878, 0" _newtrack_0) false false))))
      (:then_1
        (Utilities|FlowControl|Delay 0.7)
        (Audio|PlaySoundatLocation "/Game/Joshua/Sounds/Slidingdoor_Sounds/Sci-Fi_Sliding_Door_Cue.Sci-Fi_Sliding_Door_Cue" (Transformation|GetWorldLocation (Variables|Default|GetGlassDoorA)) "0, 0, 0" 1.0 1.0 0.0 0 0 0)))))

(fn ConstructionScript)

(fn LightStatus
  (bind _light5 (Variables|Default|GetLight5))
  (bind _light6 (Variables|Default|GetLight6))
  (bind _light7 (Variables|Default|GetLight7))
  (bind _islightred (Variables|/Game/BranMan/BranMan^2/Blueprints/Light/BP_GunLight.BP_GunLight_C|GetIsLightRed _light6))
  (bind _islightred_2 (Variables|/Game/BranMan/BranMan^2/Blueprints/Light/BP_GunLight.BP_GunLight_C|GetIsLightRed _light5))
  (bind _islightred_3 (Variables|/Game/BranMan/BranMan^2/Blueprints/Light/BP_GunLight.BP_GunLight_C|GetIsLightRed _light7))
  (bind _returnvalue (Math|Boolean|ANDBoolean _islightred_2 _islightred _islightred_3))
  (if (Math|Boolean|ANDBoolean (Variables|/Game/BranMan/BranMan^2/Blueprints/Light/BP_GunLight.BP_GunLight_C|GetIsLightRed (Variables|Default|GetLight5)) (not (Variables|/Game/BranMan/BranMan^2/Blueprints/Light/BP_GunLight.BP_GunLight_C|GetIsLightRed (Variables|Default|GetLight6))) (not (Variables|/Game/BranMan/BranMan^2/Blueprints/Light/BP_GunLight.BP_GunLight_C|GetIsLightRed (Variables|Default|GetLight7))))
    (if (Math|Boolean|ANDBoolean (Variables|/Game/BranMan/BranMan^2/Blueprints/Light/BP_GunLight.BP_GunLight_C|GetIsLightRed (Variables|Default|GetLight5)) (Variables|/Game/BranMan/BranMan^2/Blueprints/Light/BP_GunLight.BP_GunLight_C|GetIsLightRed (Variables|Default|GetLight6)) (not (Variables|/Game/BranMan/BranMan^2/Blueprints/Light/BP_GunLight.BP_GunLight_C|GetIsLightRed (Variables|Default|GetLight7))))
      (if _returnvalue
        (if _returnvalue
          (return false)
          (else
            (return true)))
        (else
          (CallFunction|SetLightsRed)))
      (else
        (CallFunction|SetLightsRed)))
    (else
      (CallFunction|SetLightsRed))))

(fn SetLightsRed
  (Variables|/Game/BranMan/BranMan^2/Blueprints/Light/BP_GunLight.BP_GunLight_C|SetIsLightRed (Variables|Default|GetLight5) true)
  (Variables|/Game/BranMan/BranMan^2/Blueprints/Light/BP_GunLight.BP_GunLight_C|SetIsLightRed (Variables|Default|GetLight6) true)
  (Variables|/Game/BranMan/BranMan^2/Blueprints/Light/BP_GunLight.BP_GunLight_C|SetIsLightRed (Variables|Default|GetLight7) true))